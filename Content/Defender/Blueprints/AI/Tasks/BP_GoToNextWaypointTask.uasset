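; Behavior Tree task that moves a soldier pawn to the next point on its looping waypoint route.
; It fails immediately if the pawn is in dialogue, and succeeds without moving if the route is empty.
; The destination comes from the soldier's world-space waypoints, indexed by a Blackboard value.
; Whether the move succeeds or fails, it advances the index with wraparound and reports success.
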(event `self.ReceiveExecuteAI`
  (params (OwnerController :type "AIController Object Reference") (ControlledPawn :type "Pawn Object Reference"))
  (set `self.Controlled Pawn` ControlledPawn)
  (bind _output_get (set `self.ControlledPawnDialogueComp` (`Actor.GetComponentByClass` (`self.Controlled Pawn`) "/Game/Defender/Blueprints/Components/DialogueComp.DialogueComp_C")))
  (`/Engine/EditorBlueprintResources/StandardMacros.IsValid` _output_get
    (:`Is Valid`
      (if (`/Game/Defender/Blueprints/Components/DialogueComp.InDialogue` (`self.ControlledPawnDialogueComp`))
        (`self.FinishExecute` false)
        (else
          (bind _output_get_2 (set `self.WaypointsWorld` (`/Game/Defender/Blueprints/Characters/BP_SoldierCharParent.WaypointsWorld` (cast `/Game/Defender/Blueprints/Characters/BP_SoldierCharParent` (`self.Controlled Pawn`) :!pure true)) :!label _label))
          (bind _output_get_3 (set `self.WaypointsLength` (`KismetArrayLibrary.Array_Length` _output_get_2)))
          (if (> _output_get_3 0)
            (bind _output_get_4 (set `self.Destination` (`|GetArrayItem` (`self.WaypointsWorld`) (`self.GetWaypointIndex`))))
            (`|AIMoveTo` (`self.Controlled Pawn`) _output_get_4 null 10.0 true
              (:`OnSuccess`
                _)
              (:`OnFail`
                _))
            (`self.SetWaypointIndex` (`KismetMathLibrary.SelectInt` 0 (+ (`self.GetWaypointIndex`) 1) (>= (+ (`self.GetWaypointIndex`) 1) (`self.WaypointsLength`))))
            (`self.FinishExecute` true)
            (else
              (`self.FinishExecute` true))))))
    (:`Is Not Valid`
      (goto _label))))

(fn `GetWaypointIndex`
  (returns (ReturnValue :type Integer))
  (return (`BTFunctionLibrary.GetBlackboardValueAsInt` (`self.WaypointIndex`))))

(fn `SetWaypointIndex`
  (params (Value :type Integer))
  (`BTFunctionLibrary.SetBlackboardValueAsInt` (`self.WaypointIndex`) Value))