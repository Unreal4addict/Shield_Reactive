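; Behavior tree task for the sniper AI that fires the equipped weapon at the blackboard TargetActor each tick.
; A capsule trace from the muzzle checks for friends with identical tags in the line of fire, stopping fire and, after a delay, switching to the bomb-throwing state.
; An empty magazine switches State to reload, and a target with assault prevention stops fire and changes State, both aborting the task.
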(event `self.ReceiveExecuteAI`
  (params (OwnerController :type "AIController Object Reference") (ControlledPawn :type "Pawn Object Reference"))
  (set `self.ControlledPawn` ControlledPawn)
  (set `self.WeaponComp` (`Actor.GetComponentByClass` (`self.ControlledPawn`) "/Game/Defender/Blueprints/Components/WeaponComp.WeaponComp_C"))
  (set `self.InventoryComp` (`Actor.GetComponentByClass` (`self.ControlledPawn`) "/Game/Defender/Blueprints/Components/InventoryComp.InventoryComp_C"))
  (set `self.RotInterp` (`Actor.K2_GetActorRotation` (`self.ControlledPawn`)))
  (set `self.ControlledPawnTags` (`Actor.Tags` (`self.ControlledPawn`)))
  (add `/Game/Defender/Blueprints/Components/WeaponComp.OnMagazineEmpty` (`self.WeaponComp`) (delegate `OnMagazineEmpty_Event_0`)) ; Reload weapon if magazine is empty
)

(event `OnMagazineEmpty_Event_0`
  (`BTFunctionLibrary.SetBlackboardValueAsEnum` (`self.State`) (enumliteral `/Game/Defender/StructsAndEnums/AiStateEnum` "NewEnumerator2"))
  (`self.FinishAbort`))

(event `self.ReceiveTickAI`
  (params (OwnerController :type "AIController Object Reference") (ControlledPawn :type "Pawn Object Reference") (DeltaSeconds :type "Float (single-precision)"))
  (set `self.Controlled Pawn` ControlledPawn)
  (if (`self.CheckValidationForTick`)
    (if (`/Game/Defender/Blueprints/Components/HealthComp.HasAssaultPreventation` (`Actor.GetComponentByClass` (`self.GetTargetActor`) "/Game/Defender/Blueprints/Components/HealthComp.HealthComp_C"))
      (`/Game/Defender/Blueprints/Components/WeaponComp.StopFiring` (`self.WeaponComp`))
      (`BTFunctionLibrary.SetBlackboardValueAsEnum` (`self.State`) (enumliteral `/Game/Defender/StructsAndEnums/AiStateEnum` "NewEnumerator9"))
      (`self.FinishAbort`)
      (else
        (bind _outhit (`KismetSystemLibrary.CapsuleTraceSingleForObjects` (`SceneComponent.K2_GetComponentLocation` (`/Game/Defender/Blueprints/Weapons/BP_WeaponParent.Muzzle` (`/Game/Defender/Blueprints/Components/InventoryComp.EquippedWeapon` (`self.InventoryComp`)))) (`self.GetTargetActorLocation`) 50.0 50.0 (`|MakeArray` "ObjectTypeQuery8" :!type "EObjectTypeQuery Enum") false (`|MakeArray` (`self.ControlledPawn`) :!type "Actor Object Reference"))) ; For checking friends in shooting route
        (bind _output_get (set `self.Hit Actor` (`.HitActor` (`GameplayStatics.BreakHitResult` _outhit))))
        (`/Engine/EditorBlueprintResources/StandardMacros.IsValid` _output_get
          (:`Is Valid`
            (if (`KismetArrayLibrary.Array_Identical` (`self.ControlledPawnTags`) (`Actor.Tags` (`self.Hit Actor`)))
              (`/Game/Defender/Blueprints/Components/WeaponComp.StopFiring` (`self.WeaponComp`))
              (`KismetSystemLibrary.Delay` 1.0)
              (`BTFunctionLibrary.SetBlackboardValueAsEnum` (`self.State`) (enumliteral `/Game/Defender/StructsAndEnums/AiStateEnum` "NewEnumerator6")) ; Change to ThrowingBomb State if condition met
              (else
                (`/Game/Defender/Blueprints/Components/WeaponComp.StartFiring` (`self.WeaponComp`) (`self.GetTargetActorLocation`)))))
          (:`Is Not Valid`
            (`/Game/Defender/Blueprints/Components/WeaponComp.StartFiring` (`self.WeaponComp`) (`self.GetTargetActorLocation`))))))))

(fn `CheckIsThereFriendInArea`
  (params (SpherePos :type "Vector Structure") (SphereRadius :type "Float (double-precision)" :default 700.0))
  (returns (Return :type Boolean))
  (locals (Location :type "Vector Structure") (Radius :type "Float (double-precision)" :default 700.0))
  (set `local.Location` SpherePos)
  (set `local.Radius` SphereRadius)
  (bind (_outactors _returnvalue) (`KismetSystemLibrary.SphereOverlapActors` (`local.Location`) (`local.Radius`) (`|MakeArray` "ObjectTypeQuery8" :!type "EObjectTypeQuery Enum") "/Game/Defender/Blueprints/Characters/BP_SoldierCharParent.BP_SoldierCharParent_C"))
  (return _returnvalue))

(fn `CheckValidationForTick`
  (returns (ReturnValue :type Boolean))
  (return (and (`KismetSystemLibrary.IsValid` (`self.WeaponComp`)) (`KismetSystemLibrary.IsValid` (`self.InventoryComp`)) (`KismetSystemLibrary.IsValid` (`self.GetTargetActor`)) (`KismetSystemLibrary.IsValid` (`/Game/Defender/Blueprints/Components/InventoryComp.EquippedWeapon` (`self.InventoryComp`))))))

(fn `GetEquippedWeapon`
  (params (ControlledPawn :type "Pawn Object Reference"))
  (returns (EquippedWeapon :type "/Game/Defender/Blueprints/Weapons/BP_WeaponParent Object Reference"))
  (return null))

(fn `GetTargetActor`
  (returns (AsActor :type "Actor Object Reference"))
  (return (cast `Actor` (`BlackboardComponent.GetValueAsObject` (`AIBlueprintHelperLibrary.GetBlackboard` (`self.Controlled Pawn`)) "TargetActor") :!pure true)))

(fn `GetTargetActorLocation`
  (returns (ReturnValue :type "Vector Structure"))
  (return (`Actor.K2_GetActorLocation` (`self.GetTargetActor`))))