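; Behavior Tree task that turns off the laser sight on the AI-controlled pawn's equipped weapon.
; On execute it gets the weapon component from the pawn, calls DeactivateLazerSight if a weapon is equipped, and finishes successfully either way.
; Helpers for the blackboard target, tick validation and soldier overlap checks are defined but unused by the event graph, and GetEquippedWeapon is an empty stub.
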(event `self.ReceiveExecuteAI`
  (params (OwnerController :type "AIController Object Reference") (ControlledPawn :type "Pawn Object Reference"))
  (set `self.ControlledPawn` ControlledPawn)
  (bind _output_get (set `self.WeaponComp` (`Actor.GetComponentByClass` (`self.ControlledPawn`) "/Game/Defender/Blueprints/Components/WeaponComp.WeaponComp_C")))
  (bind _equippedweapon (`/Game/Defender/Blueprints/Components/WeaponComp.GetInvEquippedWeapon` _output_get))
  (`/Engine/EditorBlueprintResources/StandardMacros.IsValid` _equippedweapon
    (:`Is Valid`
      (`/Game/Defender/Blueprints/Weapons/BP_WeaponParent.DeactivateLazerSight` _equippedweapon)
      (`self.FinishExecute` true))
    (:`Is Not Valid`
      (`self.FinishExecute` true))))

(fn `CheckIsThereFriendInArea`
  (params (SpherePos :type "Vector Structure") (SphereRadius :type "Float (double-precision)" :default 700.0))
  (returns (Return :type Boolean))
  (locals (Location :type "Vector Structure") (Radius :type "Float (double-precision)" :default 700.0))
  (set `local.Location` SpherePos)
  (set `local.Radius` SphereRadius)
  (bind (_outactors _returnvalue) (`KismetSystemLibrary.SphereOverlapActors` (`local.Location`) (`local.Radius`) (`|MakeArray` "ObjectTypeQuery8" :!type "EObjectTypeQuery Enum") "/Game/Defender/Blueprints/Characters/BP_SoldierCharParent.BP_SoldierCharParent_C"))
  (return _returnvalue))

(fn `CheckValidationForTick`
  (returns (ReturnValue :type Boolean))
  (return (and (`KismetSystemLibrary.IsValid` (`self.WeaponComp`)) (`KismetSystemLibrary.IsValid` (`self.InventoryComp`)) (`KismetSystemLibrary.IsValid` (`self.GetTargetActor`)) (`KismetSystemLibrary.IsValid` (`/Game/Defender/Blueprints/Components/InventoryComp.EquippedWeapon` (`self.InventoryComp`))))))

(fn `GetEquippedWeapon`
  (params (ControlledPawn :type "Pawn Object Reference"))
  (returns (EquippedWeapon :type "/Game/Defender/Blueprints/Weapons/BP_WeaponParent Object Reference"))
  (return null))

(fn `GetTargetActor`
  (returns (AsActor :type "Actor Object Reference"))
  (return (cast `Actor` (`BlackboardComponent.GetValueAsObject` (`AIBlueprintHelperLibrary.GetBlackboard` (`self.Controlled Pawn`)) "TargetActor") :!pure true)))

(fn `GetTargetActorLocation`
  (returns (ReturnValue :type "Vector Structure"))
  (return (`Actor.K2_GetActorLocation` (`self.GetTargetActor`))))