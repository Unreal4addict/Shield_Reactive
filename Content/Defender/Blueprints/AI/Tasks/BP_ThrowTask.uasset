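; Behavior tree task that makes an AI pawn throw a grenade at its blackboard target actor.
; It passes the target's location and the pawn's skeletal mesh to the pawn's ThrowComp, then finishes successfully when that component signals the throw has ended.
; During cooldown it succeeds immediately, while an invalid target leaves the task without a finish call.
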(event `self.ReceiveExecuteAI`
  (params (OwnerController :type "AIController Object Reference") (ControlledPawn :type "Pawn Object Reference"))
  (set `self.Controlled Pawn` ControlledPawn)
  (bind _output_get (set `self.ThrowComp` (`Actor.GetComponentByClass` (`self.Controlled Pawn`) "/Game/Defender/Blueprints/Components/ThrowComp.ThrowComp_C"))) ; Get Throw Component
  (if (not (`/Game/Defender/Blueprints/Components/ThrowComp.IsInThrowCooldown` _output_get))
    (bind _output_get_2 (set `self.TargetActorRef` (`BTFunctionLibrary.GetBlackboardValueAsActor` (`self.TargetActor`))))
    (`/Engine/EditorBlueprintResources/StandardMacros.IsValid` _output_get_2
      (:`Is Valid`
        (set `/Game/Defender/Blueprints/Components/ThrowComp.TargetLocation` (`Actor.K2_GetActorLocation` (`self.TargetActorRef`)) (`self.ThrowComp`)) ; Get Target Actor Location
        (`/Game/Defender/Blueprints/Components/ThrowComp.ThrowStart` (`self.ThrowComp`) (`Actor.GetComponentByClass` (`self.Controlled Pawn`) "/Script/Engine.SkeletalMeshComponent")) ; Call ThrowStart Event From\nThrow Component
        (add `/Game/Defender/Blueprints/Components/ThrowComp.OnThrowEnded` (`self.ThrowComp`) (delegate `OnThrowEnded_Event_0`))))
    (else
      (`self.FinishExecute` true))))

(event `OnThrowEnded_Event_0`
  (`self.FinishExecute` true))