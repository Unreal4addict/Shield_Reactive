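; Behavior tree task for AI soldiers that fires the equipped weapon at the blackboard target.
; On execute it switches State to throw a grenade if not reloading, grenades remain and no soldier overlaps the target area, otherwise it finishes.
; Each tick it capsule-traces from the muzzle, holding fire and changing State when a same-tag friend blocks the shot.
; An empty magazine or assault-protected target changes State and aborts.
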(event `self.ReceiveExecuteAI`
  (params (OwnerController :type "AIController Object Reference") (ControlledPawn :type "Pawn Object Reference"))
  (set `self.ControlledPawn` ControlledPawn)
  (set `self.WeaponComp` (`Actor.GetComponentByClass` (`self.ControlledPawn`) "/Game/Defender/Blueprints/Components/WeaponComp.WeaponComp_C"))
  (set `self.InventoryComp` (`Actor.GetComponentByClass` (`self.ControlledPawn`) "/Game/Defender/Blueprints/Components/InventoryComp.InventoryComp_C"))
  (set `self.RotInterp` (`Actor.K2_GetActorRotation` (`self.ControlledPawn`)))
  (set `self.ControlledPawnTags` (`Actor.Tags` (`self.ControlledPawn`)))
  (remove `/Game/Defender/Blueprints/Components/WeaponComp.OnMagazineEmpty` (`self.WeaponComp`) (delegate `OnMagazineEmpty_Event_0`))
  (add `/Game/Defender/Blueprints/Components/WeaponComp.OnMagazineEmpty` (`self.WeaponComp`) (delegate `OnMagazineEmpty_Event_0`)) ; Reload weapon if magazine is empty
  (`KismetSystemLibrary.Delay` 0.2)
  (if (not (`/Game/Defender/Blueprints/Components/WeaponComp.IsReloading` (`self.WeaponComp`)))
    (if (== (`KismetMathLibrary.RandomIntegerInRange` 1 1) 1)
      (if (> (`/Game/Defender/Blueprints/Components/InventoryComp.GrenadeCount` (`self.InventoryComp`)) 0)
        (if (not (`self.CheckIsThereFriendInArea` (`self.GetTargetActorLocation`) 1000.0))
          (`BTFunctionLibrary.SetBlackboardValueAsEnum` (`self.State`) (enumliteral `/Game/Defender/StructsAndEnums/AiStateEnum` "NewEnumerator5")) ; Change to ThrowingBomb State if condition met
          (else
            (`self.FinishExecute` true) ; It is necessary to finish execute for \nbehavior tree to continue
          ))
        (else
          (`self.FinishExecute` true) ; It is necessary to finish execute for \nbehavior tree to continue
        ))
      (else
        (`self.FinishExecute` true) ; It is necessary to finish execute for \nbehavior tree to continue
      ))
    (else
      (`self.FinishExecute` true) ; It is necessary to finish execute for \nbehavior tree to continue
    )))

(event `OnMagazineEmpty_Event_0`
  (`BTFunctionLibrary.SetBlackboardValueAsEnum` (`self.State`) (enumliteral `/Game/Defender/StructsAndEnums/AiStateEnum` "NewEnumerator2"))
  (`self.FinishAbort`))

(event `self.ReceiveTickAI`
  (params (OwnerController :type "AIController Object Reference") (ControlledPawn :type "Pawn Object Reference") (DeltaSeconds :type "Float (single-precision)"))
  (set `self.ControlledPawn` ControlledPawn)
  (if (`self.CheckValidationForTick`)
    (set `self.TargetActorLocation` (`self.GetTargetActorLocation`))
    (if (`/Game/Defender/Blueprints/Components/HealthComp.HasAssaultPreventation` (`Actor.GetComponentByClass` (`self.GetTargetActor`) "/Game/Defender/Blueprints/Components/HealthComp.HealthComp_C"))
      (`/Game/Defender/Blueprints/Components/WeaponComp.StopFiring` (`self.WeaponComp`))
      (`BTFunctionLibrary.SetBlackboardValueAsEnum` (`self.State`) (enumliteral `/Game/Defender/StructsAndEnums/AiStateEnum` "NewEnumerator9"))
      (`self.FinishAbort`)
      (else
        (bind _outhit (`KismetSystemLibrary.CapsuleTraceSingleForObjects` (`SceneComponent.K2_GetComponentLocation` (`/Game/Defender/Blueprints/Weapons/BP_WeaponParent.Muzzle` (`/Game/Defender/Blueprints/Components/InventoryComp.EquippedWeapon` (`self.InventoryComp`)))) (`self.TargetActorLocation`) 50.0 50.0 (`|MakeArray` "ObjectTypeQuery8" :!type "EObjectTypeQuery Enum") false (`|MakeArray` (`self.ControlledPawn`) :!type "Actor Object Reference"))) ; For checking friends in shooting route
        (bind _output_get (set `self.Hit Actor` (`.HitActor` (`GameplayStatics.BreakHitResult` _outhit))))
        (`/Engine/EditorBlueprintResources/StandardMacros.IsValid` _output_get
          (:`Is Valid`
            (if (`KismetArrayLibrary.Array_Identical` (`self.ControlledPawnTags`) (`Actor.Tags` (`self.Hit Actor`)))
              (`/Game/Defender/Blueprints/Components/WeaponComp.StopFiring` (`self.WeaponComp`))
              (`KismetSystemLibrary.Delay` 1.0)
              (`BTFunctionLibrary.SetBlackboardValueAsEnum` (`self.State`) (enumliteral `/Game/Defender/StructsAndEnums/AiStateEnum` "NewEnumerator6")) ; Change to ThrowingBomb State if condition met
              (else
                (`/Game/Defender/Blueprints/Components/WeaponComp.StartFiring` (`self.WeaponComp`) (`self.TargetActorLocation`)))))
          (:`Is Not Valid`
            (`/Game/Defender/Blueprints/Components/WeaponComp.StartFiring` (`self.WeaponComp`) (`self.TargetActorLocation`))))))))

(fn `CheckIsThereFriendInArea`
  (params (SpherePos :type "Vector Structure") (SphereRadius :type "Float (double-precision)" :default 700.0))
  (returns (Return :type Boolean))
  (locals (Location :type "Vector Structure") (Radius :type "Float (double-precision)" :default 700.0))
  (set `local.Location` SpherePos)
  (set `local.Radius` SphereRadius)
  (bind (_outactors _returnvalue) (`KismetSystemLibrary.SphereOverlapActors` (`local.Location`) (`local.Radius`) (`|MakeArray` "ObjectTypeQuery8" :!type "EObjectTypeQuery Enum") "/Game/Defender/Blueprints/Characters/BP_SoldierCharParent.BP_SoldierCharParent_C"))
  (return _returnvalue))

(fn `CheckValidationForTick`
  (returns (ReturnValue :type Boolean))
  (return (and (`KismetSystemLibrary.IsValid` (`self.WeaponComp`)) (`KismetSystemLibrary.IsValid` (`self.InventoryComp`)) (`KismetSystemLibrary.IsValid` (`self.GetTargetActor`)) (`KismetSystemLibrary.IsValid` (`/Game/Defender/Blueprints/Components/InventoryComp.EquippedWeapon` (`self.InventoryComp`))))))

(fn `GetTargetActor`
  (returns (AsActor :type "Actor Object Reference"))
  (return (cast `Actor` (`BlackboardComponent.GetValueAsObject` (`AIBlueprintHelperLibrary.GetBlackboard` (`self.ControlledPawn`)) "TargetActor") :!pure true)))

(fn `GetTargetActorLocation`
  (returns (ReturnValue :type "Vector Structure"))
  (bind _asactor (`self.GetTargetActor`))
  (`/Engine/EditorBlueprintResources/StandardMacros.IsValid` _asactor
    (:`Is Valid`
      (return (`Actor.K2_GetActorLocation` _asactor)))))