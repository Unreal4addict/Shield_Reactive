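; Behavior Tree task that plays a configurable montage, from a given starting section, on the controlled pawn's skeletal mesh component.
; A DoOnce gate blocks re-entry while the montage plays and resets when it ends.
; The task finishes successfully on completion, and also on interruption after a short delay.
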(event `self.ReceiveExecuteAI`
  (params (OwnerController :type "AIController Object Reference") (ControlledPawn :type "Pawn Object Reference"))
  (set `self.Controlled Pawn` ControlledPawn)
  (`/Engine/EditorBlueprintResources/StandardMacros.DoOnce` false :!label _label
    (:`Completed`
      (`|PlayMontage` (`Actor.GetComponentByClass` (`self.Controlled Pawn`) "/Script/Engine.SkeletalMeshComponent") (`self.MontageToPlay`) 1.0 0.0 (`self.MontageStartingSection`)
        (:`OnCompleted`
          _)
        (:`OnInterrupted`
          (`KismetSystemLibrary.Delay` 0.2)))
      (`self.ResetMontagePlay`)
      (`self.FinishExecute` true))))

(event `ResetMontagePlay`
  (goto _label :!via `Reset`))