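; BP_ShellParent is a shell actor, by name a parent class, that is flung from its owner and later dissolves.
; On BeginPlay it randomizes its pitch and yaw, then applies a velocity-change impulse to its static mesh, upward and opposite the owner's forward vector with random variation.
; After a fixed delay, DissolveComp runs the dissolve on that mesh.
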(event `self.ReceiveBeginPlay`
  (bind (_returnvalue_x _returnvalue_y) (`KismetMathLibrary.BreakVector` (* (`self.OwnerForwardVector`) -100.0)))
  (bind _output_get (set `self.RandomizedRotation` (`KismetMathLibrary.RandomFloatInRange` -30.0 30.0)))
  (`self.K2_SetActorRelativeRotation` (`KismetMathLibrary.MakeRotator` 0.0 _output_get _output_get))
  (set `self.OwnerForwardVector` (`KismetMathLibrary.GetForwardVector` (`self.K2_GetActorRotation` (`self.GetOwner`))))
  (set `self.RandomizedImpulse` (`KismetMathLibrary.RandomFloatInRange` -15.0 15.0))
  (`PrimitiveComponent.AddImpulse` (`self.StaticMesh`) (`KismetMathLibrary.MakeVector` (+ (`self.RandomizedImpulse`) _returnvalue_x) (+ (`self.RandomizedImpulse`) _returnvalue_y) (`KismetMathLibrary.RandomFloatInRange` 200.0 350.0)) "None" true)
  (`KismetSystemLibrary.Delay` 7.0)
  (`/Game/Defender/Blueprints/Components/DissolveComp.Execute` (`self.DissolveComp`) (`self.StaticMesh`)))

(fn `UserConstructionScript`)