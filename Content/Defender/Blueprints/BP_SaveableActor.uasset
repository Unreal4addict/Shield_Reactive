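; BP_SaveableActor is an actor Blueprint that saves and restores health state through a save game.
; SaveActor writes class, transform, health and max health into the Saveables map, keyed by object name, only when a HealthComp exists.
; LoadActor applies the saved health as a delta through ChangeHealth, then sets max health.
; It does not apply the saved transform.
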(fn `LoadActor`
  (params (SaveableStruct :type "/Game/Defender/Blueprints/SaveGames/SaveGameStructs/SaveablesStruct Structure"))
  (locals (OwnerHealthComp :type "/Game/Defender/Blueprints/Components/HealthComp Object Reference") (Struct :type "/Game/Defender/Blueprints/SaveGames/SaveGameStructs/SaveablesStruct Structure"))
  (set `local.Struct` SaveableStruct)
  (bind _output_get (set `local.OwnerHealthComp` (`self.GetComponentByClass` "/Game/Defender/Blueprints/Components/HealthComp.HealthComp_C")))
  (`/Engine/EditorBlueprintResources/StandardMacros.IsValid` _output_get
    (:`Is Valid`
      (`/Game/Defender/Blueprints/Components/HealthComp.ChangeHealth` (`local.OwnerHealthComp`) (- (`.Health_31_A58AD067423B665B196086A0F7BC9B2B` (break `/Game/Defender/Blueprints/SaveGames/SaveGameStructs/SaveablesStruct` (`local.Struct`))) (`/Game/Defender/Blueprints/Components/HealthComp.Health` (`local.OwnerHealthComp`))))
      (`/Game/Defender/Blueprints/Components/HealthComp.SetMaxHealth` (`local.OwnerHealthComp`) (`.MaxHealth_32_34D0229F474F1A7FB9F9D09221530623` (break `/Game/Defender/Blueprints/SaveGames/SaveGameStructs/SaveablesStruct` (`local.Struct`)))))))

(fn `SaveActor`
  (params (SaveGame :type "/Game/Defender/Blueprints/SaveGames/SG_Saveables Object Reference"))
  (locals (SG :type "/Game/Defender/Blueprints/SaveGames/SG_Saveables Object Reference") (OwnerHealthComp :type "/Game/Defender/Blueprints/Components/HealthComp Object Reference") (ObjectName :type String) (Class :type "/Game/Defender/Blueprints/BP_SaveableActor Class Reference") (Transform :type "Transform Structure") (Health :type "Float (double-precision)" :default 0.0) (MaxHealth :type "Float (double-precision)" :default 0.0))
  (set `local.SG` SaveGame)
  (set `local.ObjectName` (`KismetSystemLibrary.GetObjectName` self))
  (set `local.Class` (`GameplayStatics.GetObjectClass` self))
  (set `local.Transform` (`self.GetTransform`))
  (bind _output_get (set `local.OwnerHealthComp` (`self.GetComponentByClass` "/Game/Defender/Blueprints/Components/HealthComp.HealthComp_C")))
  (`/Engine/EditorBlueprintResources/StandardMacros.IsValid` _output_get
    (:`Is Valid`
      (set `local.Health` (`/Game/Defender/Blueprints/Components/HealthComp.Health` (`local.OwnerHealthComp`)))
      (set `local.MaxHealth` (`/Game/Defender/Blueprints/Components/HealthComp.MaxHealth` (`local.OwnerHealthComp`)))
      (`BlueprintMapLibrary.Map_Add` (`/Game/Defender/Blueprints/SaveGames/SG_Saveables.Saveables` (`local.SG`)) (`local.ObjectName`) (make `/Game/Defender/Blueprints/SaveGames/SaveGameStructs/SaveablesStruct` (`local.Class`) (`local.Transform`) (`local.Health`) (`local.MaxHealth`) false (struct :`UsingWeaponSlot` "NewEnumerator3") (struct) (struct :`Participant` (struct) :`DialogueType` "NewEnumerator0"))))))

(fn `UserConstructionScript`)