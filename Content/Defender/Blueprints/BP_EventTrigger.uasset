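; BP_EventTrigger is a one-shot box trigger actor that fires its OnEventTriggerUsed dispatcher when the player character enters it.
; Besides the overlap event, BeginPlay polls until the player character is valid, then checks twice, 0.2 seconds apart, for a player already inside the box.
; An IsUsed flag blocks repeat firing, and LoadActor restores it from an event trigger struct.
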(event `self.ReceiveBeginPlay`
  (`/Engine/EditorBlueprintResources/StandardMacros.IsValid` (`GameplayStatics.GetPlayerCharacter` 0) :!label _label
    (:`Is Valid`
      (if (`self.CheckIsOverlappingPlayer`)
        (`self.TriggerEvent`))
      (`KismetSystemLibrary.Delay` 0.2)
      (if (`self.CheckIsOverlappingPlayer`)
        (`self.TriggerEvent`)))
    (:`Is Not Valid`
      (`KismetSystemLibrary.Delay` 0.2) ; Wait for player character object reference\nto be valid
      (goto _label))))

(event `self.Box.OnComponentBeginOverlap`
  (params (OverlappedComponent :type "PrimitiveComponent Object Reference") (OtherActor :type "Actor Object Reference") (OtherComp :type "PrimitiveComponent Object Reference") (OtherBodyIndex :type Integer) (bFromSweep :type Boolean) (SweepResult :type "HitResult Structure (by ref)"))
  (if (== OtherActor (`GameplayStatics.GetPlayerCharacter` 0))
    (`self.TriggerEvent`)))

(fn `CheckIsOverlappingPlayer`
  (returns (OverlappingPlayer :type Boolean))
  (return (`PrimitiveComponent.IsOverlappingActor` (`self.Box`) (`GameplayStatics.GetPlayerCharacter` 0))))

(fn `LoadActor`
  (params (EventTriggersStruct :type "/Game/Defender/Blueprints/SaveGames/SaveGameStructs/EventTriggersStruct Structure"))
  (set `self.IsUsed` (`.IsUsed_1_A32EA73744F36CCD9E051186596E3B58` (break `/Game/Defender/Blueprints/SaveGames/SaveGameStructs/EventTriggersStruct` EventTriggersStruct))))

(fn `TriggerEvent`
  (if (not (`self.IsUsed`))
    (set `self.IsUsed` true)
    (`self.OnEventTriggerUsed`)))

(fn `UserConstructionScript`)