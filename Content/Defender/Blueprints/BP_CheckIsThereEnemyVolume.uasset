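; A box volume that periodically checks whether living enemies are inside it and reports when the area is cleared.
; A looping timer drives checks that gather overlapping soldiers, melee characters and turrets, excluding dialogue NPCs, and keep those alive by health component.
; Each check broadcasts the result through a dispatcher.
; Consecutive empty checks are counted to confirm a clear, then it fires the all-cleared dispatcher, stops the timer and unbinds listeners.
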(event `StartChecking`
  (`KismetSystemLibrary.Delay` 0.2)
  (bind _returnvalue (`KismetSystemLibrary.K2_SetTimerDelegate` (`|CreateDelegate` :!event `CheckIsThereEnemy`) (`self.TimeIntervalBetweenChecks`) true))
  (set `self.Timer` _returnvalue))

(fn `CheckAllEnemiesAreCleared`
  (bind _result (`/Engine/EditorBlueprintResources/StandardMacros.IncrementInt` (`self.AllEnemiesAreClearedCount`))
    (:`  `
      (if (== _result 3)
        (`self.OnAllEnemiesAreCleared`)
        (`self.StopChecking`)))))

(fn `CheckIsThereEnemy`
  (locals (InOverlappingSoldiers :type "Array of Actor Object Reference") (InOverlappingMeleeChars :type "Array of Actor Object Reference") (InAllEnemies :type "Array of Actor Object Reference") (InArrayActor :type "Actor Object Reference") (InAllAliveEnemies :type "Array of Actor Object Reference") (InIsThereAliveEnemy :type Boolean) (InOverlappingTurrets :type "Array of Actor Object Reference"))
  (`|ExecutionSequence`
    (:`then_0`
      (set `local.InOverlappingSoldiers` (`self.RemoveDialogueNPCs` (`PrimitiveComponent.GetOverlappingActors` (`self.Box`) "/Game/Defender/Blueprints/Characters/BP_SoldierCharParent.BP_SoldierCharParent_C")))
      (set `local.InOverlappingMeleeChars` (`PrimitiveComponent.GetOverlappingActors` (`self.Box`) "/Game/Defender/Blueprints/Characters/BP_MeleeCharParent.BP_MeleeCharParent_C"))
      (set `local.InOverlappingTurrets` (`PrimitiveComponent.GetOverlappingActors` (`self.Box`) "/Game/Defender/Demo/Blueprints/BP_TurretParent.BP_TurretParent_C")))
    (:`then_1`
      (`KismetArrayLibrary.Array_Append` (`local.InAllEnemies`) (`local.InOverlappingSoldiers`))
      (`KismetArrayLibrary.Array_Append` (`local.InAllEnemies`) (`local.InOverlappingMeleeChars`))
      (`KismetArrayLibrary.Array_Append` (`local.InAllEnemies`) (`local.InOverlappingTurrets`)))
    (:`then_2`
      (for _array_element (`local.InAllEnemies`)
        (bind _output_get (set `local.InArrayActor` _array_element))
        (if (`/Game/Defender/Blueprints/Components/HealthComp.isAlive` (`self.GetComponentByClass` _output_get "/Game/Defender/Blueprints/Components/HealthComp.HealthComp_C"))
          (`KismetArrayLibrary.Array_Add` (`local.InAllAliveEnemies`) (`local.InArrayActor`))
          (`KismetSystemLibrary.PrintString` (`KismetSystemLibrary.GetDisplayName` (`local.InArrayActor`)) false true (struct :`G` 0.66 :`B` 1.0 :`A` 1.0) 1.0)))
      (if (> (`KismetArrayLibrary.Array_Length` (`local.InAllAliveEnemies`)) 0)
        (bind _output_get_2 (set `local.InIsThereAliveEnemy` true))
        (`self.OnCheckIsThereEnemy` _output_get_2)
        (set `self.AllEnemiesAreClearedCount` 0) ; There is a enemy so reset AllEnemiesAreClearedCount
        (else
          (bind _output_get_3 (set `local.InIsThereAliveEnemy` false))
          (`self.OnCheckIsThereEnemy` _output_get_3)
          (`self.CheckAllEnemiesAreCleared`))))))

(fn `RemoveDialogueNPCs`
  (params (Soldiers :type "Array of Actor Object Reference"))
  (returns (OutSoldiers :type "Array of Actor Object Reference"))
  (locals (InSoldiers :type "Array of Actor Object Reference") (OutSoldierActors :type "Array of Actor Object Reference") (InArrayElement :type "Actor Object Reference"))
  (bind _output_get (set `local.InSoldiers` Soldiers))
  (for _array_element _output_get
    (set `local.InArrayElement` _array_element)
    (if (not (`KismetMathLibrary.ClassIsChildOf` (`GameplayStatics.GetObjectClass` (`local.InArrayElement`)) "/Game/Defender/Blueprints/Characters/BP_DialogueNPCParent.BP_DialogueNPCParent_C"))
      (`KismetArrayLibrary.Array_Add` (`local.OutSoldierActors`) (`local.InArrayElement`))))
  (return (`local.OutSoldierActors`)))

(fn `StopChecking`
  (bind _timer (`self.Timer`))
  (`KismetSystemLibrary.K2_PauseTimerHandle` _timer)
  (`KismetSystemLibrary.K2_ClearAndInvalidateTimerHandle` _timer)
  (clear `self.OnCheckIsThereEnemy`)
  (clear `self.OnAllEnemiesAreCleared`)
  (set `self.AllEnemiesAreClearedCount` 0))

(fn `UserConstructionScript`)