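; Base shield for Defender that absorbs damage into its own health pool, ignoring one damage type, and broadcasts health-change and destroyed events.
; Toggling it sets mesh visibility and collision, with a physical material override applied on activation and reset on a timer.
; Deactivation starts delayed, timer-driven incremental regeneration, which reactivation cancels.
; Reaching zero health deactivates the shield and schedules a full health restore after a delay, without reactivating it.
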(event `self.ReceiveBeginPlay`
  (add `self.OnTakeAnyDamage` (delegate `OnTakeDamage`))
  (set `self.ShieldHealth` (`self.ShieldMaxHealth`)))

(event `OnTakeDamage` :!signature `self.OnTakeAnyDamage`
  (params (DamagedActor :type "Actor Object Reference") (Damage :type "Float (single-precision)") (DamageType :type "DamageType Object Reference") (InstigatedBy :type "Controller Object Reference") (DamageCauser :type "Actor Object Reference"))
  (`self.ShieldHealthDecrease` Damage (`GameplayStatics.GetObjectClass` DamageType))
  (if (== (`self.ShieldHealth`) 0.0)
    (`self.OnShieldDestroyed`)
    (`self.SetShieldIsActive` false)
    (`KismetSystemLibrary.K2_SetTimer` null "FullyRestoreHealth" 0.1 false (`self.RestoreDelayAfterDestroyed`))))

(event `RestoreShieldHealth`
  (`self.Shield Health Restore` (`self.HealthRestoreAmount`))
  (if (== (`self.ShieldHealth`) (`self.ShieldMaxHealth`))
    (`KismetSystemLibrary.K2_ClearAndInvalidateTimerHandle` (`self.HealthTimer`))))

(event `ResetPhysMat`
  (`PrimitiveComponent.SetPhysMaterialOverride` (`self.ShieldMesh`) null))

(fn `FullyRestoreHealth`
  (set `self.ShieldHealth` (`self.ShieldMaxHealth`)))

(fn `SetRestoreHealthTimer`
  (bind _returnvalue (`KismetSystemLibrary.K2_SetTimerDelegate` (`|CreateDelegate` :!event `RestoreShieldHealth`) (`self.HealthRestoreRate`) true (`self.InitialHealthRestoreDelay`)))
  (set `self.HealthTimer` _returnvalue))

(fn `SetShieldIsActive`
  (params (IsActive :type Boolean))
  (if IsActive
    (`SceneComponent.SetVisibility` (`self.ShieldMesh`) true true)
    (`PrimitiveComponent.SetCollisionEnabled` (`self.ShieldMesh`) "QueryAndPhysics")
    (`KismetSystemLibrary.K2_ClearAndInvalidateTimerHandle` (`self.HealthTimer`))
    (`PrimitiveComponent.SetPhysMaterialOverride` (`self.ShieldMesh`) "/Game/Defender/PhysicMats/PM_Shield.PM_Shield")
    (`KismetSystemLibrary.K2_SetTimerDelegate` (`|CreateDelegate` :!event `ResetPhysMat`) 0.1 false (`self.ResetPhysMatTimer`))
    (else
      (`SceneComponent.SetVisibility` (`self.ShieldMesh`) false true)
      (`PrimitiveComponent.SetCollisionEnabled` (`self.ShieldMesh`) "NoCollision")
      (bind _returnvalue (`KismetSystemLibrary.K2_SetTimer` null "SetRestoreHealthTimer" (`self.RestoreTimeAfterDeactivation`)))
      (set `self.HealthTimer` _returnvalue))))

(fn `Shield Health Restore`
  (params (ChangeAmount :type "Float (double-precision)"))
  (bind _output_get (set `self.ShieldHealth` (`KismetMathLibrary.FClamp` (+ ChangeAmount (`self.ShieldHealth`)) 0.0 (`self.ShieldMaxHealth`))))
  (`self.OnHealthChanged` _output_get))

(fn `ShieldHealthDecrease`
  (params (DecreaseAmount :type "Float (double-precision)") (DamageType :type "DamageType Class Reference"))
  (if (and (!= DecreaseAmount 0.0) (!= DamageType (`self.DamageTypeToIgnore`)))
    (bind _output_get (set `self.ShieldHealth` (`KismetMathLibrary.Conv_IntToDouble` (`KismetMathLibrary.Round` (`KismetMathLibrary.FClamp` (- (`self.ShieldHealth`) DecreaseAmount) 0.0 (`self.ShieldMaxHealth`))))))
    (`self.OnHealthChanged` _output_get)))

(fn `UserConstructionScript`)