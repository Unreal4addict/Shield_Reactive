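; Character preview stage that shows a dummy of the main character on a turntable, animating even while paused.
; On BeginPlay it copies the player's weapons to the child-actor dummy, takes the view target, hides the HUD, caps FPS and scales spotlights by a GameMode multiplier.
; Rotation input sets a target spin that Tick interpolates and decays on dummy and turntable.
; DestroyRenderer restores view, HUD and FPS, then destroys dummy, weapons and itself.
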(event `DisableWeaponOutline`
  (bind _output_get (set `self.Equipped Weapon` (`/Game/Defender/Blueprints/Components/InventoryComp.EquippedWeapon` (`/Game/Defender/Blueprints/Characters/BP_MainCharParent.InventoryComp` (`self.Dummy`))) :!label _label))
  (`/Engine/EditorBlueprintResources/StandardMacros.IsValid` _output_get
    (:`Is Valid`
      (`PrimitiveComponent.SetRenderCustomDepth` (`/Game/Defender/Blueprints/Weapons/BP_WeaponParent.Mesh` (`self.Equipped Weapon`)) false) ; Remove weapon outline
    )
    (:`Is Not Valid`
      (`KismetSystemLibrary.Delay` 0.2)
      (goto _label))))

(event `self.ReceiveBeginPlay`
  (`|ExecutionSequence`
    (:`then_0`
      (bind _asbp_main_char_parent (cast `/Game/Defender/Blueprints/Characters/BP_MainCharParent` (`ChildActorComponent.ChildActor` (`self.DummyChildActor`))))
      (bind _output_get (set `self.Dummy` _asbp_main_char_parent))
      (`/Engine/EditorBlueprintResources/StandardMacros.IsValid` _output_get
        (:`Is Valid`
          (`self.TickDummyWhenPaused`)
          (`self.AdjustChildActorZ`)
          (`self.SetInitialDummyRotation`)
          (`self.DisableWeaponOutline`)
          (`self.EquipDummyWeapon`))))
    (:`then_1`
      (`/Engine/EditorBlueprintResources/StandardMacros.IsValid` (`self.GetPC`)
        (:`Is Valid`
          (`PlayerController.SetViewTargetWithBlend` (`self.GetPC`) self 0.0 "VTBlend_Linear" 0.0 false))))
    (:`then_2`
      (`KismetSystemLibrary.Delay` 0.1)
      (`self.ShowHideHUD` false)
      (`KismetSystemLibrary.Delay` 0.0)
      (`KismetSystemLibrary.ExecuteConsoleCommand` "t.MaxFPS 60" null))
    (:`then_3`
      (`self.ApplyLightingIntensity`))))

(event `self.ReceiveTick`
  (params (DeltaSeconds :type "Float (single-precision)"))
  (`/Engine/EditorBlueprintResources/StandardMacros.IsValid` (`self.Dummy`)
    (:`Is Valid`
      (set `self.InterpRotationToAdd` (`KismetMathLibrary.FInterpTo` (`self.InterpRotationToAdd`) (`self.TargetRotationToAdd`) (`GameplayStatics.GetWorldDeltaSeconds`) 2.0))
      (`self.K2_AddActorLocalRotation` (`self.Dummy`) (`KismetMathLibrary.MakeRotator` 0.0 0.0 (`self.InterpRotationToAdd`)) false false)
      (`SceneComponent.K2_AddLocalRotation` (`self.SM_TurnTable`) (`KismetMathLibrary.MakeRotator` 0.0 0.0 (`self.InterpRotationToAdd`)) false false)
      (`self.Slowdown`))))

(fn `AdjustChildActorZ`
  (`SceneComponent.K2_SetRelativeLocation` (`self.DummyChildActor`) (`KismetMathLibrary.MakeVector` 0.0 0.0 (* (- (.z (`.BoxExtent` (`KismetSystemLibrary.GetComponentBounds` (`self.SM_Renderer`)))) (+ (`CapsuleComponent.CapsuleHalfHeight` (`Character.CapsuleComponent` (`self.Dummy`))) (* (.z (`.BoxExtent` (`KismetSystemLibrary.GetComponentBounds` (`self.SM_TurnTable`)))) 2.0))) -1.0)) false false))

(fn `ApplyLightingIntensity`
  (set `self.IntensityMultiplier` (`/Game/Defender/Blueprints/BP_MainGameMode.RendererLightingIntensityMultiplier` (`/Game/Defender/Blueprints/BP_MyPlayerController.GetGameMode` (`self.GetPC`))))
  (`LightComponent.SetIntensity` (`self.SpotLight`) (* (`LightComponentBase.Intensity` (`self.SpotLight`)) (`self.IntensityMultiplier`)))
  (`LightComponent.SetIntensity` (`self.SpotLight1`) (* (`LightComponentBase.Intensity` (`self.SpotLight1`)) (`self.IntensityMultiplier`)))
  (`LightComponent.SetIntensity` (`self.SpotLight2`) (* (`LightComponentBase.Intensity` (`self.SpotLight2`)) (`self.IntensityMultiplier`)))
  (`LightComponent.SetIntensity` (`self.SpotLight3`) (* (`LightComponentBase.Intensity` (`self.SpotLight3`)) (`self.IntensityMultiplier`)))
  (`LightComponent.SetIntensity` (`self.SpotLight4`) (* (`LightComponentBase.Intensity` (`self.SpotLight4`)) (`self.IntensityMultiplier`))))

(fn `DestroyRenderer`
  (bind _pc (`self.GetPC`))
  (bind _equippedweapon (`/Game/Defender/Blueprints/Components/WeaponComp.GetInvEquippedWeapon` (`/Game/Defender/Blueprints/Characters/BP_MainCharParent.WeaponComp` (`self.Dummy`))))
  (bind _equippedmeleeweapon (`/Game/Defender/Blueprints/Components/MeleeComp.EquippedMeleeWeapon` (`/Game/Defender/Blueprints/Characters/BP_MainCharParent.MeleeComp` (`self.Dummy`))))
  (`|ExecutionSequence`
    (:`then_0`
      (`PlayerController.SetViewTargetWithBlend` _pc (`/Game/Defender/Blueprints/BP_MyPlayerController.GetMainChar` _pc) 0.0 "VTBlend_Linear" 0.0 false)
      (`self.ShowHideHUD` true)
      (`KismetSystemLibrary.ExecuteConsoleCommand` "t.MaxFPS 0" null))
    (:`then_1`
      (`/Engine/EditorBlueprintResources/StandardMacros.IsValid` (`self.Dummy`)
        (:`Is Valid`
          (`|ExecutionSequence`
            (:`then_0`
              (`/Engine/EditorBlueprintResources/StandardMacros.IsValid` _equippedweapon
                (:`Is Valid`
                  (`self.K2_DestroyActor` _equippedweapon))))
            (:`then_1`
              (`/Engine/EditorBlueprintResources/StandardMacros.IsValid` _equippedmeleeweapon
                (:`Is Valid`
                  (`self.K2_DestroyActor` _equippedmeleeweapon))))
            (:`then_2`
              (`self.K2_DestroyActor` (`self.Dummy`)))))))
    (:`then_2`
      (`ActorComponent.K2_DestroyComponent` (`self.BlockingActor`)))
    (:`then_3`
      (`self.K2_DestroyActor`))))

(fn `EquipDummyWeapon`
  (locals (InMainChar :type "/Game/Defender/Blueprints/Characters/BP_MainCharParent Object Reference"))
  (`/Engine/EditorBlueprintResources/StandardMacros.IsValid` (`self.GetPC`)
    (:`Is Valid`
      (set `local.InMainChar` (`/Game/Defender/Blueprints/BP_MyPlayerController.GetMainChar` (`self.Pc`)))
      (`/Engine/EditorBlueprintResources/StandardMacros.IsValid` (`local.InMainChar`)
        (:`Is Valid`
          (set `/Game/Defender/Blueprints/Components/InventoryComp.WeaponSlots` (`/Game/Defender/Blueprints/Components/InventoryComp.WeaponSlots` (`/Game/Defender/Blueprints/Characters/BP_MainCharParent.InventoryComp` (`local.InMainChar`))) (`/Game/Defender/Blueprints/Characters/BP_MainCharParent.InventoryComp` (`self.Dummy`)))
          (`/Game/Defender/Blueprints/Components/WeaponComp.EquipWeaponBySlot` (`/Game/Defender/Blueprints/Characters/BP_MainCharParent.WeaponComp` (`self.Dummy`)) (`/Game/Defender/Blueprints/Components/InventoryComp.UsingWeaponSlot` (`/Game/Defender/Blueprints/Characters/BP_MainCharParent.InventoryComp` (`local.InMainChar`))))
          (`/Engine/EditorBlueprintResources/StandardMacros.IsValid` (`/Game/Defender/Blueprints/Components/InventoryComp.EquippedWeapon` (`/Game/Defender/Blueprints/Characters/BP_MainCharParent.InventoryComp` (`self.Dummy`)))
            (:`Is Valid`
              (`PrimitiveComponent.SetRenderCustomDepth` (`/Game/Defender/Blueprints/Weapons/BP_WeaponParent.Mesh` (`/Game/Defender/Blueprints/Components/InventoryComp.EquippedWeapon` (`/Game/Defender/Blueprints/Characters/BP_MainCharParent.InventoryComp` (`self.Dummy`)))) false))))))))

(fn `GetPC`
  (returns (Pc :type "/Game/Defender/Blueprints/BP_MyPlayerController Object Reference"))
  (`/Engine/EditorBlueprintResources/StandardMacros.IsValid` (`self.Pc`) ; Valid Checking Of Player Controller. If it is valid, then we don't need to cast
    (:`Is Valid`
      _)
    (:`Is Not Valid`
      (bind _asbp_my_player_controller (cast `/Game/Defender/Blueprints/BP_MyPlayerController` (`GameplayStatics.GetPlayerController` 0))
        (:`then`
          (set `self.Pc` _asbp_my_player_controller))
        (:`CastFailed`
          (return null)))))
  (return (`self.Pc`)))

(fn `GetSkylight`
  (returns (SkyLight :type "SkyLight Object Reference"))
  (`/Engine/EditorBlueprintResources/StandardMacros.IsValid` (`self.SkyLight`)
    (:`Is Valid`
      _)
    (:`Is Not Valid`
      (bind _outactors (`GameplayStatics.GetAllActorsOfClass` "/Script/Engine.SkyLight"))
      (set `self.SkyLight` (`|GetArrayItem` _outactors))))
  (return (`self.SkyLight`)))

(fn `SetInitialDummyRotation`
  (`self.K2_SetActorRotation` (`self.Dummy`) (struct :`Yaw` -35.0) false)
  (`SceneComponent.K2_SetWorldRotation` (`self.SM_TurnTable`) (struct :`Yaw` -35.0) false false))

(fn `SetRotationOfDummy`
  (params (Value :type "Float (double-precision)"))
  (locals (NewLocalVar_0 :type "Float (double-precision)" :default 0.0))
  (set `self.TargetRotationToAdd` (`KismetMathLibrary.FClamp` (/ Value 20.0) -10.0 10.0)))

(fn `SetSkylightVisibility`
  (params (bNewVisibility :type Boolean))
  (`/Engine/EditorBlueprintResources/StandardMacros.IsValid` (`self.GetSkylight`)
    (:`Is Valid`
      (`SceneComponent.SetVisibility` (`SkyLight.LightComponent` (`self.SkyLight`)) bNewVisibility false))))

(fn `ShowHideHUD`
  (params (Show :type Boolean))
  (`/Engine/EditorBlueprintResources/StandardMacros.IsValid` (`/Game/Defender/Blueprints/BP_MyPlayerController.MainHUD` (`self.GetPC`))
    (:`Is Valid`
      (if Show
        (`Widget.SetVisibility` (`/Game/Defender/Blueprints/BP_MyPlayerController.MainHUD` (`self.GetPC`)) "Visible")
        (else
          (`Widget.SetVisibility` (`/Game/Defender/Blueprints/BP_MyPlayerController.MainHUD` (`self.GetPC`)) "Hidden"))))))

(fn `Slowdown`
  (if (> (`self.TargetRotationToAdd`) 1.0)
    (set `self.TargetRotationToAdd` (- (`self.TargetRotationToAdd`) 1.0))
    (elif (< (`self.TargetRotationToAdd`) -1.0)
      (set `self.TargetRotationToAdd` (+ (`self.TargetRotationToAdd`) 1.0))
      (else
        (set `self.TargetRotationToAdd` 0.0)))))

(fn `TickDummyWhenPaused`
  (`self.SetTickableWhenPaused` (`self.Dummy`) true)
  (`ActorComponent.SetTickableWhenPaused` (`Character.Mesh` (`self.Dummy`)) true)
  (for _array_element (`self.K2_GetComponentsByClass` (`self.Dummy`) "/Script/Engine.ActorComponent")
    (`ActorComponent.SetTickableWhenPaused` _array_element true)))

(fn `TrackDummy`
  (set `CineCameraComponent.FocusSettings` (make `CameraFocusSettings` "Tracking" 100000.0 (make `CameraTrackingFocusSettings` (`|ConvertAsset` (`self.Dummy`)))) (`self.CineCamera`)))

(fn `UserConstructionScript`
  (set `CineCameraComponent.CurrentFocalLength` 50.0 (`self.CineCamera`)))