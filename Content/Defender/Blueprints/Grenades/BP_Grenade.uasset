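; BP_Grenade is a thrown grenade actor that explodes on a fixed timer.
; On BeginPlay it enables physics on the mesh, applies a precomputed launch impulse, waits briefly, then calls Explode.
; Explode spawns particles and sound, fires a radial force, applies radial damage and destroys the actor.
; The camera shake is centered on the first player's view target rather than on the blast.
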(event `self.ReceiveBeginPlay`
  (`KismetSystemLibrary.Delay` 0.0)
  (`PrimitiveComponent.SetCollisionEnabled` (`self.GrenadeMesh`) "PhysicsOnly")
  (`PrimitiveComponent.SetSimulatePhysics` (`self.GrenadeMesh`) true)
  (`PrimitiveComponent.AddImpulse` (`self.GrenadeMesh`) (`self.Impulse`) "None" false) ; Add impulse according to calculated velocity
  (`KismetSystemLibrary.Delay` 2.5)
  (`self.Explode`) ; Explode after delay
)

(event `Explode`
  (set `self.GrenadeLocation` (`SceneComponent.K2_GetComponentLocation` (`self.GrenadeMesh`)))
  (`GameplayStatics.SpawnEmitterAtLocation` "/Game/Defender/Demo/Particles/P_Explosion.P_Explosion" (`self.GrenadeLocation`) (struct) (3.0 3.0 3.0) true "AutoRelease")
  (`RadialForceComponent.FireImpulse` (`self.RadialForce`)) ; Fire impulse to physic simulated meshes
  (`GameplayStatics.ApplyRadialDamage` (`self.Base Damage`) (`self.GrenadeLocation`) (`self.GrenadeRadius`) "/Script/Engine.DamageType" (`|MakeArray`) self (`self.GetInstigatorController`)) ; Apply radial damage to all actors in range
  (`GameplayStatics.PlayWorldCameraShake` "/Game/Defender/Blueprints/CameraShakes/BP_ExplosionShake.BP_ExplosionShake_C" (`self.K2_GetActorLocation` (`Controller.GetViewTarget` (`GameplayStatics.GetPlayerController` 0))) 3000.0 5000.0) ; Shake camera a bit
  (`GameplayStatics.PlaySoundAtLocation` "/Game/Defender/Demo/Audio/Other/SCue_Explosion.SCue_Explosion" (`self.K2_GetActorLocation`) (struct) 1.0 1.0 0.0 "/Game/Defender/Demo/Audio/Attenuations/ATT_Explosions.ATT_Explosions" null null)
  (`self.K2_DestroyActor`))

(fn `UserConstructionScript`)