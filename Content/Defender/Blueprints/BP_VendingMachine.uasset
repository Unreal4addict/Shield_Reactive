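; BP_VendingMachine is an interactable vending machine that opens a vending screen after the player holds the interaction input.
; A timeline, rate-scaled to InteractionDuration, fills the widget component's progress bar, retrying shortly if that widget is not yet valid.
; Early release stops the timeline and resets and hides the bar.
; On completion, it passes itself to ShowVendingWidget on the lazily cached BP_MyPlayerController.
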(event `self.ReceiveBeginPlay`
  (`|ExecutionSequence`
    (:`then_0`
      (set `self.ProgressWb` (`/Game/Defender/Blueprints/Components/ProgressWidgetComp.GetProgressWb` (`self.ProgressWidgetComp`))))
    (:`then_1`
      (`TimelineComponent.SetPlayRate` (`self.InteractionTimeline`) (`/Game/Defender/Blueprints/Libraries/BP_StandardLibrary.CalculateTimelinePlayRateByDuration` (`self.InteractionDuration`))))))

(event `/Game/Defender/Blueprints/Interfaces/BPI_InteractionInterface.InteractionPressed`
  (params (Interactor :type "Actor Object Reference"))
  (`self.StartProgressTimer`))

(event `/Game/Defender/Blueprints/Interfaces/BPI_InteractionInterface.InteractionReleased`
  (params (Interactor :type "Actor Object Reference"))
  (`self.ReleasedBeforeOpen`))

(event `StartProgressTimer`
  (`/Engine/EditorBlueprintResources/StandardMacros.IsValid` (`self.ProgressWb`) :!label _label
    (:`Is Valid`
      (`Widget.SetVisibility` (`self.ProgressWb`) "Visible")
      (bind (_direction _percent) (`Timeline|InteractionTimeline` :!via `PlayFromStart` :!label _label_2)
        (:`Update`
          (`/Game/Defender/Blueprints/WidgetBP/WB_Progress.ChangePercent` (`self.ProgressWb`) _percent))
        (:`Finished`
          (`KismetSystemLibrary.Delay` 0.2)
          (`Widget.SetVisibility` (`self.ProgressWb`) "Hidden")
          (`self.OpenVendingScreen`))))
    (:`Is Not Valid`
      (`KismetSystemLibrary.Delay` 0.2)
      (goto _label))))

(event `StopTimer`
  (goto _label_2 :!via `Stop`))

(event `ReleasedBeforeOpen`
  (`TimelineComponent.Stop` (`self.InteractionTimeline`))
  (`/Game/Defender/Blueprints/WidgetBP/WB_Progress.ChangePercent` (`self.ProgressWb`) 0.0)
  (`Widget.SetVisibility` (`self.ProgressWb`) "Hidden"))

(event `OpenVendingScreen`
  (`/Game/Defender/Blueprints/BP_MyPlayerController.ShowVendingWidget` (`self.GetPC`) self))

(fn `GetPC`
  (returns (Pc :type "/Game/Defender/Blueprints/BP_MyPlayerController Object Reference"))
  (`/Engine/EditorBlueprintResources/StandardMacros.IsValid` (`self.Pc`) ; Valid Checking Of Player Controller. If it is valid, then we don't need to cast
    (:`Is Valid`
      _)
    (:`Is Not Valid`
      (bind _asbp_my_player_controller (cast `/Game/Defender/Blueprints/BP_MyPlayerController` (`GameplayStatics.GetPlayerController` 0))
        (:`then`
          (set `self.Pc` _asbp_my_player_controller))
        (:`CastFailed`
          (return null)))))
  (return (`self.Pc`)))

(fn `UserConstructionScript`)