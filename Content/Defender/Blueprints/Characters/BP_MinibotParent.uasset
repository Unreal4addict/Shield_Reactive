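; BP_MinibotParent is the base Blueprint for floating minibots with a spotlight and cone mesh.
; A timeline bobs the mesh vertically while HealthComp reports it alive.
; On death, the mesh switches to physics with an impulse along the shot direction, plus explosion effects and sound.
; Delayed steps then clear the custom-depth outline, hide the light and cone, and run DissolveComp, destroying the actor once the dissolve completes.
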(event `self.ReceiveBeginPlay`
  (`self.Float`))

(event `self.HealthComp.OnDeath`
  (params (BoneName :type Name) (ShotFromDirection :type "Vector Structure") (HitComponent :type "PrimitiveComponent Object Reference") (InstigatedBy :type "Controller Object Reference") (DamageCauser :type "Actor Object Reference"))
  (`PrimitiveComponent.SetSimulatePhysics` (`self.Mesh`) true)
  (`PrimitiveComponent.AddImpulse` (`self.Mesh`) (* ShotFromDirection 3.0) BoneName false)
  (`GameplayStatics.SpawnEmitterAttached` "/Game/Defender/Demo/Particles/P_Explosion.P_Explosion" (`self.Mesh`) BoneName (0.0 0.0 0.0) (struct) (3.0 3.0 3.0))
  (`KismetSystemLibrary.K2_SetTimer` null "RemoveOutline" 2.0) ; Timer for removing outline
  (`GameplayStatics.PlaySoundAtLocation` "/Game/Defender/Demo/Audio/Other/SCue_Explosion.SCue_Explosion" (`self.K2_GetActorLocation`) (struct) 1.0 1.0 0.0 null null null)
  (`KismetSystemLibrary.Delay` 5.0)
  (`SceneComponent.SetVisibility` (`self.SpotLight`) false false)
  (`SceneComponent.SetVisibility` (`self.ConeSM`) false false)
  (`/Game/Defender/Blueprints/Components/DissolveComp.Execute` (`self.DissolveComp`) (`self.Mesh`))
  (add `/Game/Defender/Blueprints/Components/DissolveComp.DissolveCompleted` (`self.DissolveComp`) (delegate `DissolveCompleted_Event_0`)))

(event `DissolveCompleted_Event_0`
  (`self.K2_DestroyActor`))

(event `Float`
  (bind (_direction _newtrack_0) (`Timeline|Timeline_0` :!via `PlayFromStart`)
    (:`Update`
      (if (`/Game/Defender/Blueprints/Components/HealthComp.isAlive` (`self.HealthComp`))
        (`SceneComponent.K2_SetRelativeLocation` (`self.Mesh`) (`KismetMathLibrary.MakeVector` 0.0 0.0 (`KismetMathLibrary.Lerp` 250.0 300.0 _newtrack_0)) false false)))))

(fn `RemoveOutline`
  (`PrimitiveComponent.SetRenderCustomDepth` (`self.Mesh`) false) ; Remove outline
)

(fn `UserConstructionScript`)