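; BP_MeleeCharParent is a parent Blueprint for AI-controlled melee characters, built from health, stats, melee, dissolve and ragdoll components.
; On death it limits capsule collision to WorldStatic, stops AI logic, optionally ragdolls using hit data, and later clears the outline and dissolves before destruction.
; LoadActor restores transform, health, stats and melee data from a saved struct.
; Construction places the XP text at the capsule's half height.
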(event `self.HealthComp.OnDeath`
  (params (BoneName :type Name) (ShotFromDirection :type "Vector Structure") (HitComponent :type "PrimitiveComponent Object Reference") (InstigatedBy :type "Controller Object Reference") (DamageCauser :type "Actor Object Reference"))
  (bind _returnvalue (`AIBlueprintHelperLibrary.GetAIController` self))
  (set `self.BoneName` BoneName)
  (set `self.ShotFromDirection` ShotFromDirection)
  (set `self.Hit Component` HitComponent)
  (`|ExecutionSequence`
    (:`then_0`
      (`PrimitiveComponent.SetCollisionResponseToAllChannels` (`self.CapsuleComponent`) "ECR_Ignore")
      (`PrimitiveComponent.SetCollisionResponseToChannel` (`self.CapsuleComponent`) "ECC_WorldStatic" "ECR_Block") ; For standing in game world\nwe must capsule comp collide with floor
      (`Controller.StopMovement` _returnvalue)
      (`BrainComponent.StopLogic` (`AIController.BrainComponent` _returnvalue) "")
      (`KismetSystemLibrary.K2_SetTimer` null "RemoveOutline" 2.0) ; Timer for removing outline
    )
    (:`then_1`
      (`KismetSystemLibrary.Delay` 5.0)
      (`/Game/Defender/Blueprints/Components/DissolveComp.Execute` (`self.DissolveComp`) (`self.Mesh`))
      (add `/Game/Defender/Blueprints/Components/DissolveComp.DissolveCompleted` (`self.DissolveComp`) (`|CreateDelegate` :!event `DissolveCompleted`)))
    (:`then_2`
      (if (`self.IsRagdollEnabledOnDeath`)
        (`/Game/Defender/Blueprints/Components/RagdollComp.Execute` (`self.RagdollComp`) (`self.CapsuleComponent`) (`self.Mesh`) (`self.Hit Component`) (`self.BoneName`) (`self.ShotFromDirection`))))))

(fn `DissolveCompleted`
  (`self.K2_DestroyActor`))

(fn `LoadActor`
  (params (MeleeCharStruct :type "/Game/Defender/Blueprints/SaveGames/SaveGameStructs/MeleeCharsStruct Structure"))
  (locals (InStruct :type "/Game/Defender/Blueprints/SaveGames/SaveGameStructs/MeleeCharsStruct Structure") (EquippedWeapon :type "/Game/Defender/Blueprints/Weapons/BP_WeaponParent Object Reference") (StatsCompData :type "/Game/Defender/Blueprints/SaveGames/SaveGameStructs/SaveGameStatsCompStruct Structure") (MeleeCompData :type "/Game/Defender/Blueprints/SaveGames/SaveGameStructs/SaveGameMeleeCompStruct Structure"))
  (bind ((`Health_13_1C2B531547491A35E801F9A9FD7C7C6C` _health) (`MaxHealth_12_8C00E5014A8BF03AC36787B28DE23C2E` _maxhealth)) (break `/Game/Defender/Blueprints/SaveGames/SaveGameStructs/MeleeCharsStruct` (`local.InStruct`)))
  (set `local.InStruct` MeleeCharStruct)
  (set `local.StatsCompData` (`.StatsCompData_50_8AD29FFA4DEC6290963FF5BD7F135FFC` (break `/Game/Defender/Blueprints/SaveGames/SaveGameStructs/MeleeCharsStruct` (`local.InStruct`))))
  (set `local.MeleeCompData` (`.MeleeCompData_57_4D4510A64F74BCC34C902D93A1C55DDD` (break `/Game/Defender/Blueprints/SaveGames/SaveGameStructs/MeleeCharsStruct` (`local.InStruct`))))
  (`self.K2_SetActorTransform` (`.Transform_14_E6D0EC384EA76DAE00B0498F7DBC69BD` (break `/Game/Defender/Blueprints/SaveGames/SaveGameStructs/MeleeCharsStruct` (`local.InStruct`))))
  (`/Game/Defender/Blueprints/Components/StatsComp.LoadData` (`self.StatsComp`) (`local.StatsCompData`))
  (`/Game/Defender/Blueprints/Components/MeleeComp.LoadData` (`self.MeleeComp`) (`local.MeleeCompData`))
  (`self.SetHealthMaxHealth` _health _maxhealth))

(fn `RemoveOutline`
  (`PrimitiveComponent.SetRenderCustomDepth` (`self.Mesh`) false) ; Remove outline
)

(fn `SetHealthMaxHealth`
  (params (Health :type "Float (double-precision)") (MaxHealth :type "Float (double-precision)"))
  (locals (OldHealth :type "Float (double-precision)" :default 0.0) (NewHealth :type "Float (double-precision)") (NewMaxHealth :type "Float (double-precision)"))
  (set `local.NewHealth` Health)
  (set `local.NewMaxHealth` MaxHealth)
  (set `local.OldHealth` (`/Game/Defender/Blueprints/Components/HealthComp.Health` (`self.HealthComp`)))
  (`/Game/Defender/Blueprints/Components/HealthComp.ChangeHealth` (`self.HealthComp`) (- (`local.NewHealth`) (`local.OldHealth`)))
  (`/Game/Defender/Blueprints/Components/HealthComp.SetMaxHealth` (`self.HealthComp`) (`local.NewMaxHealth`)))

(fn `UserConstructionScript`
  (`SceneComponent.K2_SetRelativeLocation` (`self.XPTextComp`) (`KismetMathLibrary.MakeVector` 0.0 0.0 (`CapsuleComponent.CapsuleHalfHeight` (`self.CapsuleComponent`))) false false))