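; Parent Blueprint for soldier characters, handling death, restoring saved state and waypoint setup.
; On death it ragdolls from the hit, plays a sound, clears the outline on a timer, then dissolves after a randomized delay and destroys itself.
; LoadActor restores transform, health, stats, inventory and equipped weapon, plus dialogue and melee components if present.
; The construction script converts local waypoints to world locations and places XP text at capsule half-height.
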(event `self.HealthComp.OnDeath`
  (params (BoneName :type Name) (ShotFromDirection :type "Vector Structure") (HitComponent :type "PrimitiveComponent Object Reference") (InstigatedBy :type "Controller Object Reference") (DamageCauser :type "Actor Object Reference"))
  (`/Game/Defender/Blueprints/Components/RagdollComp.Execute` (`self.RagdollComp`) (`self.CapsuleComponent`) (`self.Mesh`) HitComponent BoneName ShotFromDirection) ; Execute Ragdoll because of death
  (`GameplayStatics.PlaySoundAtLocation` (`self.DeathSound`) (`self.K2_GetActorLocation`) (struct) 1.0 1.0 0.0 null null null)
  (`KismetSystemLibrary.K2_SetTimer` null "RemoveOutline" 2.0) ; Timer for removing outline
  (`KismetSystemLibrary.Delay` (+ (`self.DissolveStartDelay`) (`KismetMathLibrary.RandomFloatInRange` 1.0 3.0)))
  (`/Game/Defender/Blueprints/Components/DissolveComp.Execute` (`self.DissolveComp`) (`self.Mesh`)) ; Execute Dissolve because of death
)

(event `self.DissolveComp.DissolveCompleted`
  (`self.K2_DestroyActor`) ; Destroy Actor when dissolve completed
)

(fn `DestroyEquippedWeapon`
  (bind _equippedweapon (`/Game/Defender/Blueprints/Components/InventoryComp.EquippedWeapon` (`self.InventoryComp`)))
  (`/Engine/EditorBlueprintResources/StandardMacros.IsValid` _equippedweapon
    (:`Is Valid`
      (`self.K2_DestroyActor` _equippedweapon))))

(fn `GetPC`
  (returns (Pc :type "/Game/Defender/Blueprints/BP_MyPlayerController Object Reference"))
  (`/Engine/EditorBlueprintResources/StandardMacros.IsValid` (`self.Pc`) ; Get player controller reference once, if it is valid
    (:`Is Valid`
      _)
    (:`Is Not Valid`
      (bind _asbp_my_player_controller (cast `/Game/Defender/Blueprints/BP_MyPlayerController` (`GameplayStatics.GetPlayerController` 0))
        (:`then`
          (set `self.Pc` _asbp_my_player_controller))
        (:`CastFailed`
          (return null)))))
  (return (`self.Pc`)))

(fn `LoadActor`
  (params (EnemiesStruct :type "/Game/Defender/Blueprints/SaveGames/SaveGameStructs/SoldiersStruct Structure"))
  (locals (Struct :type "/Game/Defender/Blueprints/SaveGames/SaveGameStructs/SoldiersStruct Structure") (EquippedWeapon :type "/Game/Defender/Blueprints/Weapons/BP_WeaponParent Object Reference") (InventoryCompData :type "/Game/Defender/Blueprints/SaveGames/SaveGameStructs/SaveGameInventoryStruct Structure") (StatsCompData :type "/Game/Defender/Blueprints/SaveGames/SaveGameStructs/SaveGameStatsCompStruct Structure") (InDialogueComp :type "/Game/Defender/Blueprints/Components/DialogueComp Object Reference") (InMeleeComp :type "/Game/Defender/Blueprints/Components/MeleeComp Object Reference"))
  (bind ((`Health_13_1C2B531547491A35E801F9A9FD7C7C6C` _health) (`MaxHealth_12_8C00E5014A8BF03AC36787B28DE23C2E` _maxhealth)) (break `/Game/Defender/Blueprints/SaveGames/SaveGameStructs/SoldiersStruct` (`local.Struct`)))
  (set `local.Struct` EnemiesStruct)
  (`|ExecutionSequence`
    (:`then_0`
      (`self.K2_SetActorTransform` (`.Transform_14_E6D0EC384EA76DAE00B0498F7DBC69BD` (break `/Game/Defender/Blueprints/SaveGames/SaveGameStructs/SoldiersStruct` (`local.Struct`))))
      (`self.SetHealthMaxHealth` _health _maxhealth))
    (:`then_1`
      (set `local.StatsCompData` (`.StatsCompData_58_13837584455B3BACBA5EE3A71C2AEC4C` (break `/Game/Defender/Blueprints/SaveGames/SaveGameStructs/SoldiersStruct` (`local.Struct`))))
      (`/Game/Defender/Blueprints/Components/StatsComp.LoadData` (`self.StatsComp`) (`local.StatsCompData`)))
    (:`then_2`
      (set `local.InventoryCompData` (`.InventoryCompData_59_BC09D769495E2E5CE8956AB804EC2A8F` (break `/Game/Defender/Blueprints/SaveGames/SaveGameStructs/SoldiersStruct` (`local.Struct`))))
      (`/Game/Defender/Blueprints/Components/InventoryComp.LoadData` (`self.InventoryComp`) (`local.InventoryCompData`))
      (bind _equippedweapon (`/Game/Defender/Blueprints/Components/WeaponComp.EquipWeapon` (`self.WeaponComp`) (`BlueprintMapLibrary.Map_Find` (`/Game/Defender/Blueprints/Components/InventoryComp.WeaponSlots` (`self.InventoryComp`)) (`.UsingWeaponSlot_44_BF88B6DD4C3E8D2B5D851F864F9C1629` (break `/Game/Defender/Blueprints/SaveGames/SaveGameStructs/SaveGameInventoryStruct` (`local.InventoryCompData`)))) (`self.Mesh`)))
      (set `local.EquippedWeapon` _equippedweapon)
      (`/Game/Defender/Blueprints/Weapons/BP_WeaponParent.SetMagazineAmmo` (`local.EquippedWeapon`) (`/Game/Defender/Blueprints/Weapons/BP_WeaponParent.GetMagazineAmmo` (`local.EquippedWeapon`))))
    (:`then_3`
      (bind _output_get (set `local.InDialogueComp` (`self.GetComponentByClass` "/Game/Defender/Blueprints/Components/DialogueComp.DialogueComp_C")))
      (`/Engine/EditorBlueprintResources/StandardMacros.IsValid` _output_get
        (:`Is Valid`
          (`/Game/Defender/Blueprints/Components/DialogueComp.LoadData` (`local.InDialogueComp`) (`.DialogueCompData_63_37A6117B4857DA2B5E6D358E9B197FCE` (break `/Game/Defender/Blueprints/SaveGames/SaveGameStructs/SoldiersStruct` (`local.Struct`)))))))
    (:`then_4`
      (bind _output_get_2 (set `local.InMeleeComp` (`self.GetComponentByClass` "/Game/Defender/Blueprints/Components/MeleeComp.MeleeComp_C")))
      (`/Engine/EditorBlueprintResources/StandardMacros.IsValid` _output_get_2
        (:`Is Valid`
          (`/Game/Defender/Blueprints/Components/MeleeComp.LoadData` (`local.InMeleeComp`) (`.MeleeCompData_69_FDEA57774FAEAC223DA22D9B13C497A3` (break `/Game/Defender/Blueprints/SaveGames/SaveGameStructs/SoldiersStruct` (`local.Struct`)))))))))

(fn `ProjectWaypointsToWorldLocs`
  (for _array_element (`self.Waypoints`)
    (`KismetArrayLibrary.Array_Add` (`self.WaypointsWorld`) (`KismetMathLibrary.TransformLocation` (`self.GetTransform`) _array_element))))

(fn `RemoveOutline`
  (`PrimitiveComponent.SetRenderCustomDepth` (`self.Mesh`) false) ; Remove outline
)

(fn `SetHealthMaxHealth`
  (params (Health :type "Float (double-precision)") (MaxHealth :type "Float (double-precision)"))
  (locals (OldHealth :type "Float (double-precision)" :default 0.0) (NewHealth :type "Float (double-precision)") (NewMaxHealth :type "Float (double-precision)"))
  (set `local.NewHealth` Health)
  (set `local.NewMaxHealth` MaxHealth)
  (set `local.OldHealth` (`/Game/Defender/Blueprints/Components/HealthComp.Health` (`self.HealthComp`)))
  (`/Game/Defender/Blueprints/Components/HealthComp.ChangeHealth` (`self.HealthComp`) (- (`local.NewHealth`) (`local.OldHealth`)))
  (`/Game/Defender/Blueprints/Components/HealthComp.SetMaxHealth` (`self.HealthComp`) (`local.NewMaxHealth`)))

(fn `UserConstructionScript`
  (`self.ProjectWaypointsToWorldLocs`)
  (`SceneComponent.K2_SetRelativeLocation` (`self.XPTextComp`) (`KismetMathLibrary.MakeVector` 0.0 0.0 (`CapsuleComponent.CapsuleHalfHeight` (`self.CapsuleComponent`))) false false))