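; Anim notify state that marks the melee hit window in Defender attack animations.
; On begin, it finds the owner's MeleeComp, calls StrikeStart and enables its melee trace flag.
; On end, it disables the flag and calls StrikeEnd, leaving the trace logic itself to the component.
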(fn `Received_NotifyBegin`
  (params (MeshComp :type "SkeletalMeshComponent Object Reference") (Animation :type "AnimSequenceBase Object Reference") (TotalDuration :type "Float (double-precision)"))
  (returns (ReturnValue :type Boolean))
  (locals (InOwner :type "Actor Object Reference") (InMeleeComp :type "/Game/Defender/Blueprints/Components/MeleeComp Object Reference"))
  (set `local.InOwner` (`ActorComponent.GetOwner` MeshComp))
  (bind _output_get (set `local.InMeleeComp` (`Actor.GetComponentByClass` (`local.InOwner`) "/Game/Defender/Blueprints/Components/MeleeComp.MeleeComp_C")))
  (`/Engine/EditorBlueprintResources/StandardMacros.IsValid` _output_get
    (:`Is Valid`
      (`/Game/Defender/Blueprints/Components/MeleeComp.StrikeStart` (`local.InMeleeComp`))
      (set `/Game/Defender/Blueprints/Components/MeleeComp.IsMeleeTraceEnabled` true (`local.InMeleeComp`))
      (return true))))

(fn `Received_NotifyEnd`
  (params (MeshComp :type "SkeletalMeshComponent Object Reference") (Animation :type "AnimSequenceBase Object Reference"))
  (returns (ReturnValue :type Boolean))
  (locals (InOwner :type "Actor Object Reference") (InMeleeComp :type "/Game/Defender/Blueprints/Components/MeleeComp Object Reference"))
  (set `local.InOwner` (`ActorComponent.GetOwner` MeshComp))
  (bind _output_get (set `local.InMeleeComp` (`Actor.GetComponentByClass` (`local.InOwner`) "/Game/Defender/Blueprints/Components/MeleeComp.MeleeComp_C")))
  (`/Engine/EditorBlueprintResources/StandardMacros.IsValid` _output_get
    (:`Is Valid`
      (set `/Game/Defender/Blueprints/Components/MeleeComp.IsMeleeTraceEnabled` false (`local.InMeleeComp`))
      (`/Game/Defender/Blueprints/Components/MeleeComp.StrikeEnd` (`local.InMeleeComp`))
      (return false))))