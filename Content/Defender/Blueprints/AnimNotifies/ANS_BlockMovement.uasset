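; Anim notify state that freezes a character's movement for the duration of an animation window.
; On begin it sets the owner's CharacterMovement mode to None; on end it restores it to Walking, regardless of the earlier mode.
; If the owner is the first player's character, it also disables that player controller's input on begin and re-enables it on end.
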(fn `Received_NotifyBegin`
  (params (MeshComp :type "SkeletalMeshComponent Object Reference") (Animation :type "AnimSequenceBase Object Reference") (TotalDuration :type "Float (double-precision)"))
  (returns (ReturnValue :type Boolean))
  (locals (InOwner :type "Actor Object Reference") (InMeleeComp :type "/Game/Defender/Blueprints/Components/MeleeComp Object Reference") (Mesh :type "SkeletalMeshComponent Object Reference") (OwnerActor :type "Actor Object Reference") (CharacterMovementComp :type "CharacterMovementComponent Object Reference") (PC :type "PlayerController Object Reference"))
  (bind _pc (`local.PC`))
  (set `local.Mesh` MeshComp)
  (bind _output_get (set `local.OwnerActor` (`ActorComponent.GetOwner` (`local.Mesh`))))
  (`/Engine/EditorBlueprintResources/StandardMacros.IsValid` _output_get
    (:`Is Valid`
      (if (== (`local.OwnerActor`) (`GameplayStatics.GetPlayerCharacter` (`local.Mesh`)))
        (set `local.PC` (`GameplayStatics.GetPlayerController` (`local.Mesh`)))
        (`Actor.DisableInput` _pc _pc))
      (bind _output_get_2 (set `local.CharacterMovementComp` (`Actor.GetComponentByClass` (`local.OwnerActor`) "/Script/Engine.CharacterMovementComponent")))
      (`/Engine/EditorBlueprintResources/StandardMacros.IsValid` _output_get_2
        (:`Is Valid`
          (`CharacterMovementComponent.SetMovementMode` (`local.CharacterMovementComp`) "MOVE_None" 0)
          (return true))))))

(fn `Received_NotifyEnd`
  (params (MeshComp :type "SkeletalMeshComponent Object Reference") (Animation :type "AnimSequenceBase Object Reference"))
  (returns (ReturnValue :type Boolean))
  (locals (Mesh :type "SkeletalMeshComponent Object Reference") (OwnerActor :type "Actor Object Reference") (PC :type "PlayerController Object Reference") (CharacterMovementComp :type "CharacterMovementComponent Object Reference"))
  (bind _pc (`local.PC`))
  (set `local.Mesh` MeshComp)
  (bind _output_get (set `local.OwnerActor` (`ActorComponent.GetOwner` (`local.Mesh`))))
  (`/Engine/EditorBlueprintResources/StandardMacros.IsValid` _output_get
    (:`Is Valid`
      (if (== (`local.OwnerActor`) (`GameplayStatics.GetPlayerCharacter` (`local.Mesh`)))
        (set `local.PC` (`GameplayStatics.GetPlayerController` (`local.Mesh`)))
        (`Actor.EnableInput` _pc _pc))
      (bind _output_get_2 (set `local.CharacterMovementComp` (`Actor.GetComponentByClass` (`local.OwnerActor`) "/Script/Engine.CharacterMovementComponent")))
      (`/Engine/EditorBlueprintResources/StandardMacros.IsValid` _output_get_2
        (:`Is Valid`
          (`CharacterMovementComponent.SetMovementMode` (`local.CharacterMovementComp`) "MOVE_Walking" 0)
          (return true))))))