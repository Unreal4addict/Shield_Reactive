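; Anim notify that makes the animated actor deal radial damage at a chosen frame of an animation.
; When fired, it applies radial damage in a fixed radius around the mesh owner's location using the radial damage type.
; The owner is ignored by the damage and recorded as its causer, and the amount comes from the RadialDamage variable.
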(fn `GetNotifyName`
  (returns (ReturnValue :type String))
  (return "AN Radial Damage"))

(fn `Received_Notify`
  (params (MeshComp :type "SkeletalMeshComponent Object Reference") (Animation :type "AnimSequenceBase Object Reference"))
  (returns (ReturnValue :type Boolean))
  (locals (OwnerActor :type "Actor Object Reference"))
  (bind _output_get (set `local.OwnerActor` (`ActorComponent.GetOwner` MeshComp)))
  (bind _returnvalue (`GameplayStatics.ApplyRadialDamage` (`self.RadialDamage`) (`Actor.K2_GetActorLocation` _output_get) 700.0 "/Game/Defender/Blueprints/DamageTypes/BP_DamageTypeRadial.BP_DamageTypeRadial_C" (`|MakeArray` (`local.OwnerActor`)) (`local.OwnerActor`) null))
  (return _returnvalue))