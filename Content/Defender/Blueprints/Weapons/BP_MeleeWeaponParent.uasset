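; Parent Blueprint for melee weapons in the Defender game, providing a dissolve-then-destroy removal.
; DissolveWeapon runs the dissolve component on the static mesh if one is assigned, otherwise on the skeletal mesh, and binds to its completion event.
; A DissolveCompleted function destroys the actor, and the construction script resets the Box component to zero world rotation.
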(fn `DissolveCompleted`
  (`self.K2_DestroyActor`))

(fn `DissolveWeapon`
  (`/Engine/EditorBlueprintResources/StandardMacros.IsValid` (`StaticMeshComponent.StaticMesh` (`self.MeleeWeaponStaticMesh`))
    (:`Is Valid`
      (`/Game/Defender/Blueprints/Components/DissolveComp.Execute` (`self.DissolveComp`) (`self.MeleeWeaponStaticMesh`)))
    (:`Is Not Valid`
      (`/Engine/EditorBlueprintResources/StandardMacros.IsValid` (`SkinnedMeshComponent.SkeletalMesh` (`self.MeleeWeaponSkeletalMesh`))
        (:`Is Valid`
          (`/Game/Defender/Blueprints/Components/DissolveComp.Execute` (`self.DissolveComp`) (`self.MeleeWeaponSkeletalMesh`))))))
  (add `/Game/Defender/Blueprints/Components/DissolveComp.DissolveCompleted` (`self.DissolveComp`) (`|CreateDelegate` :!event `DissolveCompleted`)))

(fn `UserConstructionScript`
  (`SceneComponent.K2_SetWorldRotation` :`self` (`self.Box`)))