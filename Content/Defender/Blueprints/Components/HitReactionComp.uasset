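; Actor component that makes its owner react to damage with a sound and a random section of a hit reaction montage.
; It binds point and radial damage events, reacting only while HealthComp reports alive; point hits roll a probability, radial hits always play the montage.
; Soldier types stop firing and flag WeaponComp during the reaction.
; Turn-to-damager helpers with timed tick shutoff exist, but nothing in these graphs calls them.
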(event `self.ReceiveBeginPlay`
  (if (`self.IsEnabled`)
    (`/Engine/EditorBlueprintResources/StandardMacros.IsValid` (`self.HitReactionMontage`) ; Check if owner have a montage\nto play when hit
      (:`Is Valid`
        (set `self.OwnerActor` (`self.GetOwner`))
        (set `self.OwnerSK` (`Actor.GetComponentByClass` (`self.OwnerActor`) "/Script/Engine.SkeletalMeshComponent"))
        (add `Actor.OnTakePointDamage` (`self.OwnerActor`) (`|CreateDelegate` :!event `OnTakeDamageEvent`)) ; Bind event to take point damage.
        (add `Actor.OnTakeRadialDamage` (`self.OwnerActor`) (`|CreateDelegate` :!event `OnTakeRadialDamageEvent`)) ; Bind event to take radial damage.
      ))))

(event `OnTakeDamageEvent`
  (params (DamagedActor :type "Actor Object Reference") (Damage :type "Float (double-precision)") (InstigatedBy :type "Controller Object Reference") (HitLocation :type "Vector Structure") (FHitComponent :type "PrimitiveComponent Object Reference") (BoneName :type Name) (ShotFromDirection :type "Vector Structure") (DamageType :type "DamageType Object Reference") (DamageCauser :type "Actor Object Reference"))
  (set `self.InstigatedBy` InstigatedBy)
  (set `self.DamageCauser` DamageCauser)
  (if (`/Game/Defender/Blueprints/Components/HealthComp.isAlive` (`self.GetHealthComp`))
    (`GameplayStatics.PlaySoundAtLocation` (`self.PointDamageSound`) (`Actor.K2_GetActorLocation` (`self.OwnerActor`)) (struct) 1.0 1.0 0.0 null null null)
    (if (>= (`self.PointDamageHitReactProbability`) (`KismetMathLibrary.RandomFloatInRange` 0.0 1.0))
      (switch `/Game/Defender/StructsAndEnums/ReactHitType` (`self.ReactHitType`) :!label _label
        (:`NewEnumerator0`
          (set `/Game/Defender/Blueprints/Components/WeaponComp.IsReactHitAnimPlaying` true (`self.GetWeaponComp`))
          (`/Game/Defender/Blueprints/Components/WeaponComp.StopFiring` (`self.GetWeaponComp`)))
        (:`NewEnumerator1`
          _))
      (set `self.IsReactHitAnimPlaying` true)
      (`|PlayMontage` (`self.OwnerSK`) (`self.HitReactionMontage`) (`self.PlayRate`) 0.0 (`|GetArrayItem` (`self.HitReactionMontageSectionNames`) (`KismetMathLibrary.RandomIntegerInRange` 0 (- (`KismetArrayLibrary.Array_Length` (`self.HitReactionMontageSectionNames`)) 1))) ; Play reaction animation coming from the montage.
        (:`OnCompleted`
          (`KismetSystemLibrary.Delay` 1.0 :!label _label_2))
        (:`OnBlendOut`
          (goto _label_2))
        (:`OnInterrupted`
          _))
      (switch `/Game/Defender/StructsAndEnums/ReactHitType` (`self.ReactHitType`)
        (:`NewEnumerator0`
          (set `/Game/Defender/Blueprints/Components/WeaponComp.IsReactHitAnimPlaying` false (`self.GetWeaponComp`)))
        (:`NewEnumerator1`
          _))
      (set `self.IsReactHitAnimPlaying` false))))

(event `OnTakeRadialDamageEvent`
  (params (DamagedActor :type "Actor Object Reference") (Damage :type "Float (double-precision)") (DamageType :type "DamageType Object Reference") (Origin :type "Vector Structure") (HitInfo :type "HitResult Structure") (InstigatedBy :type "Controller Object Reference") (DamageCauser :type "Actor Object Reference"))
  (set `self.DamageCauser` DamageCauser)
  (if (`/Game/Defender/Blueprints/Components/HealthComp.isAlive` (`self.GetHealthComp`))
    (`GameplayStatics.PlaySoundAtLocation` (`self.RadialDamageSound`) (`Actor.K2_GetActorLocation` (`self.OwnerActor`)) (struct) 1.0 1.0 0.0 null null null)
    (goto _label)))

(fn `DisableComponentTick`
  (`self.SetComponentTickEnabled` false))

(fn `EnableComponentTick`
  (`self.SetComponentTickEnabled` true))

(fn `GetHealthComp`
  (returns (HealthComp :type "/Game/Defender/Blueprints/Components/HealthComp Object Reference"))
  (`/Engine/EditorBlueprintResources/StandardMacros.IsValid` (`self.HealthComp`)
    (:`Is Valid`
      _)
    (:`Is Not Valid`
      (set `self.HealthComp` (`Actor.GetComponentByClass` (`self.GetOwner`) "/Game/Defender/Blueprints/Components/HealthComp.HealthComp_C"))))
  (return (`self.HealthComp`)))

(fn `GetWeaponComp`
  (returns (Return :type "/Game/Defender/Blueprints/Components/WeaponComp Object Reference"))
  (`/Engine/EditorBlueprintResources/StandardMacros.IsValid` (`self.WeaponComp`)
    (:`Is Valid`
      _)
    (:`Is Not Valid`
      (set `self.WeaponComp` (`Actor.GetComponentByClass` (`self.GetOwner`) "/Game/Defender/Blueprints/Components/WeaponComp.WeaponComp_C"))))
  (return (`self.WeaponComp`)))

(fn `OwnerRotation`
  (set `self.OwnerCurrentRotation` (`KismetMathLibrary.RInterpTo` (`self.OwnerCurrentRotation`) (`self.OwnerTargetRotation`) (`GameplayStatics.GetWorldDeltaSeconds`) 10.0))
  (`Actor.K2_SetActorRelativeRotation` (`self.OwnerActor`) (`self.OwnerCurrentRotation`) false false))

(fn `TurnToDamagerWhenHitReacting`
  (locals (ControlledPawn :type "Pawn Object Reference"))
  (if (`self.TurnToDamager`)
    (`/Engine/EditorBlueprintResources/StandardMacros.IsValid` (`self.InstigatedBy`)
      (:`Is Valid`
        (bind _output_get (set `local.ControlledPawn` (`Controller.K2_GetPawn` (`self.InstigatedBy`))))
        (`/Engine/EditorBlueprintResources/StandardMacros.IsValid` _output_get
          (:`Is Valid`
            (set `self.OwnerTargetRotation` (`KismetMathLibrary.FindLookAtRotation` (`Actor.K2_GetActorLocation` (`self.OwnerActor`)) (`Actor.K2_GetActorLocation` (`local.ControlledPawn`))))
            (`self.SetComponentTickEnabled` true)
            (`|ExecutionSequence`
              (:`then_0`
                (if (`KismetSystemLibrary.K2_IsValidTimerHandle` (`self.DisableComponentTickTimer`))
                  (`KismetSystemLibrary.K2_ClearAndInvalidateTimerHandle` (`self.DisableComponentTickTimer`))))
              (:`then_1`
                (bind _returnvalue (`KismetSystemLibrary.K2_SetTimer` self "DisableComponentTick" 0.3))
                (set `self.DisableComponentTickTimer` _returnvalue)))))))))