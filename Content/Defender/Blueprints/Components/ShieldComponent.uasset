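; Actor component that gives its owner a directional shield, spawned inactive in front at BeginPlay and attached.
; Location and rotation helpers place the shield front, back, left or right, at spawn or when moved.
; Activation, deactivation and destruction lock use and start delay timers, with dispatchers broadcasting availability.
; Removing the shield destroys it and starts a looping timer naming RestoreOwnerHealth, which is absent here.
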(event `self.ReceiveBeginPlay`
  ;[1 1 1] Begin Play
  (`self.SpawnShieldEvent` "NewEnumerator0"))

(event `SpawnShieldEvent`
  (params (ShieldLocation :type "/Game/Defender/Blueprints/Shield/ShieldSpawnData Enum" :default "NewEnumerator0"))
  (bind _spawnedshield (`self.SpawnedShield`))
  ;[1 1 1] Shield Spawn
  (if (and (`KismetSystemLibrary.IsValidClass` (`self.ShieldType`)) (`KismetSystemLibrary.IsValid` (`self.GetOwner`)))
    (set `self.CanUseShield` true)
    (`self.SetShieldRotation` ShieldLocation)
    (`self.SetShieldLocation` ShieldLocation)
    (bind _returnvalue (`self.SpawnShield`))
    (bind _output_get (set `self.SpawnedShield` _returnvalue))
    (`/Engine/EditorBlueprintResources/StandardMacros.IsValid` _output_get
      (:`Is Valid`
        (`Actor.K2_AttachToActor` _output_get (`self.GetOwner`) "None" "KeepWorld" "KeepRelative" "KeepRelative" true)
        (add `/Game/Defender/Blueprints/Shield/BP_BaseShield.OnShieldDestroyed` (`self.SpawnedShield`) (`|CreateDelegate` :!event `OnShieldDestroyed_Event`))
        (`/Game/Defender/Blueprints/Shield/BP_BaseShield.SetShieldIsActive` (`self.SpawnedShield`) false)
        (`self.ShieldCreated`)
        (`/Game/Defender/Blueprints/Shield/BP_BaseShield.OnHealthChanged` _spawnedshield (`/Game/Defender/Blueprints/Shield/BP_BaseShield.ShieldHealth` _spawnedshield))))))

(event `DeactivateShield`
  ;[1 1 1] Shield Deactivate
  (if (`self.CanUseShield`)
    (`/Game/Defender/Blueprints/Shield/BP_BaseShield.SetShieldIsActive` (`self.SpawnedShield`) false)
    (set `self.ShieldIsActive` false)
    (set `self.CanUseShield` false)
    (`KismetSystemLibrary.K2_SetTimerDelegate` (`|CreateDelegate` :!event `SetShieldCanBeUsed`) 0.1 false (`self.DelayAfterUse`))))

(event `ActivateShield`
  ;[1 1 1] Shield Activate
  (if (and (`self.CanUseShield`) (!= (`/Game/Defender/Blueprints/Shield/BP_BaseShield.ShieldHealth` (`self.SpawnedShield`)) 0.0))
    (`/Game/Defender/Blueprints/Shield/BP_BaseShield.SetShieldIsActive` (`self.SpawnedShield`) true)
    (set `self.ShieldIsActive` true)
    (set `self.CanUseShield` false)
    (`KismetSystemLibrary.K2_SetTimerDelegate` (`|CreateDelegate` :!event `SetShieldCanBeUsed`) 0.1 false (`self.DelayAfterUse`))))

(event `OnShieldDestroyed_Event`
  ;[1 1 1] On Shield Destroyed Event
  (set `self.ShieldIsActive` false)
  (set `self.CanUseShield` false)
  (`KismetSystemLibrary.K2_SetTimerDelegate` (`|CreateDelegate` :!event `SetShieldCanBeUsed`) 0.1 false (`self.DelayAfterDestruction`))
  (`self.ShieldCantBeUsed`))

(event `SetShieldCanBeUsed`
  ;[1 1 1] Set Shield Can Be Used
  (set `self.CanUseShield` true)
  (`self.ShieldCanBeUsed`))

(fn `ChangeShieldLocation`
  (params (ShieldLocation :type "/Game/Defender/Blueprints/Shield/ShieldSpawnData Enum" :default "NewEnumerator0"))
  (`/Engine/EditorBlueprintResources/StandardMacros.IsValid` (`self.SpawnedShield`)
    (:`Is Valid`
      (`self.SetShieldRotation` ShieldLocation)
      (`self.SetShieldLocation` ShieldLocation)
      (`Actor.K2_SetActorLocation` (`self.SpawnedShield`) (`self.SpawnLocation`) false false)
      (`Actor.K2_SetActorRelativeRotation` (`self.SpawnedShield`) (`self.ShieldRotation`) false false))))

(fn `RemoveShield`
  (if (and (`KismetSystemLibrary.IsValid` (`self.SpawnedShield`)) (`self.CanUseShield`))
    (`Actor.K2_DestroyActor` (`self.SpawnedShield`))
    (`KismetSystemLibrary.K2_SetTimerDelegate` (`|CreateDelegate` :!event `SetShieldCanBeUsed`) 0.1 false (`self.DelayAfterUse`))
    (`KismetSystemLibrary.K2_SetTimer` null "RestoreOwnerHealth" 0.0 true)
    (`self.ShieldStateChanged`)))

(fn `SetShieldLocation`
  (params (Location :type "/Game/Defender/Blueprints/Shield/ShieldSpawnData Enum" :default "NewEnumerator0"))
  (switch `/Game/Defender/Blueprints/Shield/ShieldSpawnData` Location
    (:`NewEnumerator0`
      (set `self.SpawnLocation` (+ (* (`Actor.GetActorForwardVector` (`self.GetOwner`)) (`KismetMathLibrary.Conv_DoubleToVector` (`self.SpawnDistance`))) (`Actor.K2_GetActorLocation` (`self.GetOwner`))))
      (return))
    (:`NewEnumerator1`
      (set `self.SpawnLocation` (+ (* (* (`Actor.GetActorForwardVector` (`self.GetOwner`)) (`KismetMathLibrary.Conv_DoubleToVector` -1.0)) (`KismetMathLibrary.Conv_DoubleToVector` (`self.SpawnDistance`))) (`Actor.K2_GetActorLocation` (`self.GetOwner`))))
      (return))
    (:`NewEnumerator2`
      (set `self.SpawnLocation` (+ (* (`Actor.GetActorRightVector` (`self.GetOwner`)) (`KismetMathLibrary.Conv_DoubleToVector` (`self.SpawnDistance`))) (`Actor.K2_GetActorLocation` (`self.GetOwner`))))
      (return))
    (:`NewEnumerator3`
      (set `self.SpawnLocation` (+ (* (* (`Actor.GetActorRightVector` (`self.GetOwner`)) (`KismetMathLibrary.Conv_DoubleToVector` -1.0)) (`KismetMathLibrary.Conv_DoubleToVector` (`self.SpawnDistance`))) (`Actor.K2_GetActorLocation` (`self.GetOwner`))))
      (return))))

(fn `SetShieldRotation`
  (params (SpawnLocation :type "/Game/Defender/Blueprints/Shield/ShieldSpawnData Enum" :default "NewEnumerator0"))
  (switch `/Game/Defender/Blueprints/Shield/ShieldSpawnData` SpawnLocation
    (:`NewEnumerator0`
      (set `self.ShieldRotation` (struct)))
    (:`NewEnumerator1`
      (set `self.ShieldRotation` (struct :`Yaw` 180.0)))
    (:`NewEnumerator2`
      (set `self.ShieldRotation` (struct :`Yaw` 90.0)))
    (:`NewEnumerator3`
      (set `self.ShieldRotation` (struct :`Yaw` -90.0)))))

(fn `SpawnShield`
  (returns (ReturnValue :type "/Game/Defender/Blueprints/Shield/BP_BaseShield Object Reference"))
  (bind _returnvalue (`|SpawnActorFromClass` (`self.ShieldType`) (`KismetMathLibrary.MakeTransform` (`self.SpawnLocation`) (`self.ShieldRotation`) (`self.ShieldScale`)) "Undefined" "OverrideRootScale" (`self.GetOwner`) null))
  (return _returnvalue))