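; XPTextComp is a widget component that hosts a WB_XPText widget, by its name for showing XP text on the actor that owns it.
; On BeginPlay it passes the owning actor to the widget as ParentActor.
; GetWidgetComp lazily casts the component's user widget to WB_XPText and caches it in WidgetComp, which holds the widget itself despite its name.
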(event `self.ReceiveBeginPlay`
  (`/Engine/EditorBlueprintResources/StandardMacros.IsValid` (`self.GetWidgetComp`)
    (:`Is Valid`
      (set `/Game/Defender/Blueprints/WidgetBP/WB_XPText.ParentActor` (`self.GetOwner`) (`self.WidgetComp`)))))

(fn `GetWidgetComp`
  (returns (Output_Get :type "/Game/Defender/Blueprints/WidgetBP/WB_XPText Object Reference"))
  (`/Engine/EditorBlueprintResources/StandardMacros.IsValid` (`self.WidgetComp`)
    (:`Is Valid`
      _)
    (:`Is Not Valid`
      (bind _aswb_xptext (cast `/Game/Defender/Blueprints/WidgetBP/WB_XPText` (`self.GetUserWidgetObject`)))
      (set `self.WidgetComp` _aswb_xptext)))
  (return (`self.WidgetComp`)))