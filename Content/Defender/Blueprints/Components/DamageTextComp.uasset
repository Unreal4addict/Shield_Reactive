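; DamageTextComp is a widget component that hosts the WB_DamageText widget, presumably for damage and heal text on its owning actor.
; On BeginPlay it passes the owner and its own damage and heal fonts and colors to the widget, so the style is set on the component.
; GetWidgetComp lazily casts the component's user widget to WB_DamageText and caches it.
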(event `self.ReceiveBeginPlay`
  (`/Engine/EditorBlueprintResources/StandardMacros.IsValid` (`self.GetWidgetComp`)
    (:`Is Valid`
      (set `/Game/Defender/Blueprints/WidgetBP/WB_DamageText.ParentActor` (`self.GetOwner`) (`self.WidgetComp`))
      (set `/Game/Defender/Blueprints/WidgetBP/WB_DamageText.HealFontColor` (`self.HealFontColor`) (`self.WidgetComp`)) ; Transfer widget \nHealFontColor variable
      (set `/Game/Defender/Blueprints/WidgetBP/WB_DamageText.HealFont` (`self.HealFont`) (`self.WidgetComp`)) ; Transfer widget \nHealFont variable
      (set `/Game/Defender/Blueprints/WidgetBP/WB_DamageText.DamageFontColor` (`self.DamageFontColor`) (`self.WidgetComp`)) ; Transfer widget \nDamageFontColor variable
      (set `/Game/Defender/Blueprints/WidgetBP/WB_DamageText.DamageFont` (`self.DamageFont`) (`self.WidgetComp`)) ; Transfer widget \nDamageFont variable
    )))

(fn `GetWidgetComp`
  (returns (Output_Get :type "/Game/Defender/Blueprints/WidgetBP/WB_DamageText Object Reference"))
  (`/Engine/EditorBlueprintResources/StandardMacros.IsValid` (`self.WidgetComp`)
    (:`Is Valid`
      _)
    (:`Is Not Valid`
      (bind _aswb_damage_text (cast `/Game/Defender/Blueprints/WidgetBP/WB_DamageText` (`self.GetUserWidgetObject`)))
      (set `self.WidgetComp` _aswb_damage_text)))
  (return (`self.WidgetComp`)))