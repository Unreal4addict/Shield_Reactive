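; Interactor component that lets its owning actor interact with nearby actors in response to interaction input.
; On press, it sphere-overlaps around the owner and picks the first actor with an open interaction indicator that passes a reachability check.
; It sends press and release messages to that stored actor, passing the owner.
; If candidates exist but none are reachable, the lazily cached player controller shows an obstacle warning.
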(fn `GetPC`
  (returns (Pc :type "/Game/Defender/Blueprints/BP_MyPlayerController Object Reference"))
  (`/Engine/EditorBlueprintResources/StandardMacros.IsValid` (`self.Pc`) ; Valid Checking Of Player Controller. If it is valid, then we don't need to cast
    (:`Is Valid`
      _)
    (:`Is Not Valid`
      (bind _asbp_my_player_controller (cast `/Game/Defender/Blueprints/BP_MyPlayerController` (`GameplayStatics.GetPlayerController` 0))
        (:`then`
          (set `self.Pc` _asbp_my_player_controller))
        (:`CastFailed`
          (return null)))))
  (return (`self.Pc`)))

(fn `InteractionPressed`
  (locals (InOwnerActor :type "Actor Object Reference") (InteractionIndicatorWidgetComp :type "/Game/Defender/Blueprints/Components/InteractionIndicatorWidgetComp Object Reference") (InActor :type "Actor Object Reference") (Found :type Boolean) (OwnerActorLocation :type "Vector Structure" :default (0.0 0.0 0.0)) (LineTraceHitActor :type "Actor Object Reference") (InteractionActorExistButCannotReachable :type Boolean))
  (set `local.InOwnerActor` (`self.GetOwner`))
  (set `self.InteractionActor` null) ; Assign empty
  (set `local.OwnerActorLocation` (`Actor.K2_GetActorLocation` (`local.InOwnerActor`)))
  (bind _outactors (`KismetSystemLibrary.SphereOverlapActors` (`local.OwnerActorLocation`) 700.0 (`|MakeArray`) null (`|MakeArray` (`local.InOwnerActor`)))) ; Look for the actors
  (for _array_element _outactors
    (set `local.InActor` _array_element)
    (if (not (`local.Found`))
      (bind _output_get (set `local.InteractionIndicatorWidgetComp` (`Actor.GetComponentByClass` (`local.InActor`) "/Game/Defender/Blueprints/Components/InteractionIndicatorWidgetComp.InteractionIndicatorWidgetComp_C")))
      (`/Engine/EditorBlueprintResources/StandardMacros.IsValid` _output_get
        (:`Is Valid`
          (if (`/Game/Defender/Blueprints/WidgetBP/Dialogue/WB_InteractionIndicator.Opened` (`/Game/Defender/Blueprints/Components/InteractionIndicatorWidgetComp.GetInteractionIndicatorWb` (`local.InteractionIndicatorWidgetComp`)))
            (if (`/Game/Defender/Blueprints/Libraries/BP_StandardLibrary.CheckInteractionActorIsReachable` (`local.InOwnerActor`) (`local.InActor`))
              (set `local.Found` true)
              (set `self.InteractionActor` (`local.InActor`))
              (else
                (set `local.InteractionActorExistButCannotReachable` true))))))))
  (`/Engine/EditorBlueprintResources/StandardMacros.IsValid` (`self.InteractionActor`)
    (:`Is Valid`
      (`KismetSystemLibrary.PrintString` (`KismetSystemLibrary.GetDisplayName` (`self.InteractionActor`)) false)
      (message `/Game/Defender/Blueprints/Interfaces/BPI_InteractionInterface.InteractionPressed` (`self.InteractionActor`) (`local.InOwnerActor`)))
    (:`Is Not Valid`
      (if (`local.InteractionActorExistButCannotReachable`)
        (`/Game/Defender/Blueprints/BP_MyPlayerController.ShowScreenMessage` (`self.GetPC`) "There is an obstacle. Can not reach. " true)))))

(fn `InteractionReleased`
  (locals (InOwnerActor :type "Actor Object Reference"))
  (set `local.InOwnerActor` (`self.GetOwner`))
  (message `/Game/Defender/Blueprints/Interfaces/BPI_InteractionInterface.InteractionReleased` (`self.InteractionActor`) (`local.InOwnerActor`)))