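; Actor component that turns a dead character's mesh into a physics ragdoll.
; Execute switches the mesh to ragdoll collision and simulation, applies a bone impulse along the shot direction, and disables capsule gravity while changing its collision profile.
; For owners other than the player, it moves the capsule to world origin after a short delay as a collision fix.
; Later radial damage pushes the ragdoll away from the blast, with vertical force inverted and amplified.
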(event `Execute`
  (params (CapsuleComponent :type "CapsuleComponent Object Reference") (Mesh :type "SkeletalMeshComponent Object Reference") (InHitComp :type "PrimitiveComponent Object Reference") (InBoneName :type Name) (InShotFromDirection :type "Vector Structure"))
  (set `self.CapsuleComponent` CapsuleComponent)
  (set `self.Mesh` Mesh)
  (set `self.InHitComp` InHitComp)
  (set `self.InBoneName` InBoneName)
  (set `self.InShotFromDirection` InShotFromDirection)
  (`PrimitiveComponent.SetCollisionProfileName` (`self.Mesh`) "CustomRagdoll" true)
  (`PrimitiveComponent.SetCollisionEnabled` (`self.Mesh`) "QueryAndPhysics") ; Enable Physics Only Collision
  (`PrimitiveComponent.SetSimulatePhysics` (`self.Mesh`) true) ; Enable physics sim
  (add `Actor.OnTakeRadialDamage` (`self.GetOwner`) (`|CreateDelegate` :!event `OnTakeRadialDamage`))
  (`PrimitiveComponent.AddImpulse` (`self.Mesh`) (* (`self.InShotFromDirection`) (`self.ImpulseMultiplier`)) (`self.InBoneName`) false) ; Add impulse to mesh with shot from direction and \nadd impulse to mesh according to its physic asset
  (`PrimitiveComponent.SetEnableGravity` (`self.CapsuleComponent`) false)
  (`PrimitiveComponent.SetCollisionProfileName` (`self.CapsuleComponent`) "CapsuleAfterDeath" true)
  (if (!= (`self.GetOwner`) (`GameplayStatics.GetPlayerCharacter` 0))
    (`KismetSystemLibrary.Delay` 0.2)
    (`SceneComponent.K2_SetWorldLocation` (`self.CapsuleComponent`) (0.0 0.0 0.0) false true) ; Fix: Change capsule location for preventing collision issues
  ))

(event `OnTakeRadialDamage`
  (params (DamagedActor :type "Actor Object Reference") (Damage :type "Float (double-precision)") (DamageType :type "DamageType Object Reference") (Origin :type "Vector Structure") (HitInfo :type "HitResult Structure") (InstigatedBy :type "Controller Object Reference") (DamageCauser :type "Actor Object Reference"))
  (bind (_returnvalue_x _returnvalue_y _returnvalue_z) (`KismetMathLibrary.BreakVector` (* (`KismetMathLibrary.Normal` (- (`SceneComponent.K2_GetComponentLocation` (`self.Mesh`)) Origin)) 1500.0)))
  (`PrimitiveComponent.AddImpulse` (`self.Mesh`) (`KismetMathLibrary.MakeVector` _returnvalue_x _returnvalue_y (* _returnvalue_z -25.0)) "None" true))