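; Actor component that plays character animation montages and turns animation notifies into gameplay actions for its owner.
; Anim state changes start reload or grenade-toss montages, with interruption handlers cleaning up weapon, throw and reload-widget state.
; Notifies drive reload completion, grenade spawning, reverse dissolve and a once-only Gruntling suicide explosion.
; Footstep notifies trace down for the physical material, playing quieter when crouched and 2D for the player.
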(event `self.ReceiveBeginPlay`
  (set `self.OwnerActor` (`self.GetOwner`))
  (set `self.OwnerSk` (`Actor.GetComponentByClass` (`self.OwnerActor`) "/Script/Engine.SkeletalMeshComponent"))
  (set `self.ThrowComp` (`Actor.GetComponentByClass` (`self.OwnerActor`) "/Game/Defender/Blueprints/Components/ThrowComp.ThrowComp_C"))
  (set `self.WeaponComp` (`Actor.GetComponentByClass` (`self.OwnerActor`) "/Game/Defender/Blueprints/Components/WeaponComp.WeaponComp_C"))
  (set `self.InventoryComp` (`Actor.GetComponentByClass` (`self.OwnerActor`) "/Game/Defender/Blueprints/Components/InventoryComp.InventoryComp_C"))
  (add `self.OnAnimStateChanged` (`|CreateDelegate` :!event `AnimStateChanged`)))

(event `AnimStateChanged` :!signature `self.OnAnimStateChanged`
  (params (AnimState :type "/Game/Defender/StructsAndEnums/AnimState Enum" :default "NewEnumerator0"))
  (bind _output_get (set `self.AnimState` AnimState))
  (switch `/Game/Defender/StructsAndEnums/AnimState` _output_get
    (:`NewEnumerator1`
      (`Widget.SetVisibility` (`/Game/Defender/Blueprints/Components/ReloadWidgetComp.GetWidgetComp` (`self.GetReloadWidgetComp`)) "Visible")
      (`|PlayMontage` (`self.OwnerSk`) "/Game/Defender/Demo/Animations/Soldier/AM_Mannequin.AM_Mannequin" 1.0 0.0 "Reload"
        (:`OnBlendOut`
          _)
        (:`OnInterrupted`
          _))
      (`KismetSystemLibrary.Delay` 0.1)
      (`self.Reload Interrupted`))
    (:`NewEnumerator2`
      (`|PlayMontage` (`self.OwnerSk`) "/Game/Defender/Demo/Animations/Soldier/AM_Mannequin.AM_Mannequin" 1.0 0.0 "TossGrenade" :!label _label
        (:`OnInterrupted`
          (`KismetSystemLibrary.Delay` 0.1)
          (`self.TossGrenadeInterrupted`))))))

(event `ResetTossingGrenade`
  (`/Engine/EditorBlueprintResources/StandardMacros.DoOnce` false :!via `Reset`
    (:`Completed`
      (goto _label))))

(event `Notify`
  (params (NotifyName :type Name))
  (bind _inventorycomp (`self.InventoryComp`))
  (bind _equippedweapon (`/Game/Defender/Blueprints/Components/InventoryComp.EquippedWeapon` _inventorycomp))
  (switch `name` NotifyName
    (:`Default`
      (`KismetSystemLibrary.PrintString` "There is an issue in notifies (AnimComp)"))
    (:`ReloadCompleted`
      (`/Engine/EditorBlueprintResources/StandardMacros.IsValid` _inventorycomp
        (:`Is Valid`
          (`/Engine/EditorBlueprintResources/StandardMacros.IsValid` _equippedweapon
            (:`Is Valid`
              (`/Game/Defender/Blueprints/Weapons/BP_WeaponParent.Reload Completed Actions` _equippedweapon)
              (set `/Game/Defender/Blueprints/Components/WeaponComp.IsReloading` false (`self.WeaponComp`))
              (`/Game/Defender/Blueprints/Components/WeaponComp.OnReloadCompleted` (`self.WeaponComp`)))))))
    (:`ThrowGrenade`
      (`/Game/Defender/Blueprints/Components/ThrowComp.SpawnGrenade` (`self.ThrowComp`)))
    (:`ThrowEnd`
      (`/Game/Defender/Blueprints/Components/ThrowComp.ThrowEnd` (`self.ThrowComp`)))
    (:`MakeFootstep`
      (`self.Make Footsteps`))
    (:`ReverseDissolve`
      (`self.ReverseDissolve`))
    (:`GruntlingExplode`
      (`self.GruntlingExplode`))))

(fn `GetReloadWidgetComp`
  (returns (ReloadWidgetComp :type "/Game/Defender/Blueprints/Components/ReloadWidgetComp Object Reference"))
  (`/Engine/EditorBlueprintResources/StandardMacros.IsValid` (`self.ReloadWidgetComp`)
    (:`Is Valid`
      _)
    (:`Is Not Valid`
      (set `self.ReloadWidgetComp` (`Actor.GetComponentByClass` (`self.OwnerActor`) "/Game/Defender/Blueprints/Components/ReloadWidgetComp.ReloadWidgetComp_C"))))
  (return (`self.ReloadWidgetComp`)))

(fn `GruntlingExplode`
  (`/Engine/EditorBlueprintResources/StandardMacros.DoOnce` false
    (:`Completed`
      (bind _output_get (set `self.OwnerActorLocation` (`Actor.K2_GetActorLocation` (`self.OwnerActor`))))
      (`GameplayStatics.SpawnEmitterAtLocation` "/Game/Defender/Demo/Particles/P_Explosion.P_Explosion" _output_get (struct) (3.0 3.0 3.0) true "AutoRelease")
      (`GameplayStatics.ApplyRadialDamage` (`self.GruntlingExplodeDamage`) (`self.OwnerActorLocation`) 500.0 "/Script/Engine.DamageType" (`|MakeArray`) (`self.OwnerActor`) (`Actor.GetInstigatorController` (`self.OwnerActor`))) ; Apply radial damage to all actors in range
      (`GameplayStatics.ApplyPointDamage` (`self.OwnerActor`) 1000.0 (* (`KismetMathLibrary.GetForwardVector` (`Actor.K2_GetActorRotation` (`self.OwnerActor`))) -3.0) (`GameplayStatics.MakeHitResult` false) (`Actor.GetInstigatorController` (`self.OwnerActor`)) (`self.OwnerActor`) "/Script/Engine.DamageType") ; Apply point damage to self
      (`GameplayStatics.PlayWorldCameraShake` "/Game/Defender/Blueprints/CameraShakes/BP_ExplosionShake.BP_ExplosionShake_C" (`Actor.K2_GetActorLocation` (`Controller.GetViewTarget` (`GameplayStatics.GetPlayerController` 0))) 3000.0 5000.0) ; Shake camera a bit
      (`GameplayStatics.PlaySoundAtLocation` "/Game/Defender/Demo/Audio/Other/SCue_Explosion.SCue_Explosion" (`self.OwnerActorLocation`) (struct) 1.0 1.0 0.0 "/Game/Defender/Demo/Audio/Attenuations/ATT_Explosions.ATT_Explosions" null null) ; Play explosion sound
    )))

(fn `Make Footsteps`
  (locals (InActorLocation :type "Vector Structure" :default (0.0 0.0 0.0)) (InHit :type "HitResult Structure") (InFootstepSound :type "SoundBase Object Reference" :default "SoundCue'/Game/Defender/Demo/Audio/Footsteps/SCue_FS_Metal.SCue_FS_Metal'") (InVolumeMultiplier :type "Float (double-precision)" :default 1.0) (IsCrouching :type Boolean :default false))
  (bind (_inactorlocation_x _inactorlocation_y _inactorlocation_z) (`KismetMathLibrary.BreakVector` (`local.InActorLocation`)))
  (set `local.InActorLocation` (`Actor.K2_GetActorLocation` (`self.OwnerActor`)))
  (bind (_outhit _returnvalue) (`KismetSystemLibrary.LineTraceSingle` (`local.InActorLocation`) (`KismetMathLibrary.MakeVector` _inactorlocation_x _inactorlocation_y (- _inactorlocation_z 100.0)) "TraceTypeQuery1" false (`|MakeArray`)))
  (if _returnvalue
    (set `local.InHit` _outhit)
    (bind _output_get (set `local.IsCrouching` (`NavMovementComponent.IsCrouching` (`Actor.GetComponentByClass` (`self.OwnerActor`) "/Script/Engine.CharacterMovementComponent"))))
    (if _output_get
      (set `local.InVolumeMultiplier` 0.5)
      (else
        (set `local.InVolumeMultiplier` 1.0)))
    (switch `string` (`KismetSystemLibrary.GetDisplayName` (`.PhysMat` (`GameplayStatics.BreakHitResult` (`local.InHit`))))
      (:`Default`
        (set `local.InFootstepSound` "/Game/Defender/Demo/Audio/Footsteps/SCue_FS_Tile.SCue_FS_Tile"))
      (:`PM_Metal`
        (set `local.InFootstepSound` "/Game/Defender/Demo/Audio/Footsteps/SCue_FS_Metal.SCue_FS_Metal"))
      (:`PM_Grass`
        (set `local.InFootstepSound` "/Game/Defender/Demo/Audio/Footsteps/SCue_FS_Grass.SCue_FS_Grass")))
    (if (`self.IsCompOwnedByPlayer`)
      (`GameplayStatics.PlaySound2D` (`local.InFootstepSound`) (`local.InVolumeMultiplier`) 1.0 0.0 null null)
      (else
        (`GameplayStatics.PlaySoundAtLocation` (`local.InFootstepSound`) (`local.InActorLocation`) (struct) (`local.InVolumeMultiplier`) 1.0 0.0 "/Game/Defender/Demo/Audio/Attenuations/ATT_Footsteps.ATT_Footsteps" null null)))))

(fn `Reload Interrupted`
  (`/Game/Defender/Blueprints/Components/WeaponComp.StopReloading` (`self.WeaponComp`))
  (`Widget.SetVisibility` (`/Game/Defender/Blueprints/Components/ReloadWidgetComp.GetWidgetComp` (`self.GetReloadWidgetComp`)) "Hidden"))

(fn `ReverseDissolve`
  (`/Game/Defender/Blueprints/Components/DissolveComp.ReverseDissolve` (`Actor.GetComponentByClass` (`self.OwnerActor`) "/Game/Defender/Blueprints/Components/DissolveComp.DissolveComp_C") (`self.OwnerSk`)))

(fn `TossGrenadeInterrupted`
  (`/Game/Defender/Blueprints/Components/ThrowComp.ThrowEnd` (`self.ThrowComp`))
  (`self.ResetTossingGrenade`))