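; Blueprint function library that maps a hit's physical material surface type to impact feedback and damage scaling.
; Separate lookups return particle and scale or sound for projectile and melee hits, plus a decal that is currently identical for every surface.
; The damage multiplier reduces metal hits, applies a caller-supplied multiplier to vulnerable flesh such as heads, and doubles the result on critical hits.
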(fn `GetHitDamageMultiplier`
  (params (PhysicMat :type "PhysicalMaterial Object Reference") (VulnarableDamageMultiplier :type "Float (double-precision)" :default 10.0) (CriticalHit :type Boolean))
  (returns (DamageMultiplier :type "Float (double-precision)"))
  (locals (InDamageMultiplier :type "Float (double-precision)") (SurfaceType :type "EPhysicalSurface Enum" :default "SurfaceType_Default") (InVulnarableDamageMultiplier :type "Float (double-precision)" :default 10.0) (InCriticalHit :type Boolean))
  (set `local.SurfaceType` (`PhysicalMaterial.SurfaceType` PhysicMat))
  (set `local.InVulnarableDamageMultiplier` VulnarableDamageMultiplier)
  (set `local.InCriticalHit` CriticalHit)
  (switch `EPhysicalSurface` (`local.SurfaceType`)
    (:`SurfaceType_Default`
      (set `local.InDamageMultiplier` 1.0))
    (:`SurfaceType1`
      (set `local.InDamageMultiplier` 1.0))
    (:`SurfaceType2`
      (set `local.InDamageMultiplier` (`local.InVulnarableDamageMultiplier`)) ; Multiplier 10 in Flesh Vulnarable eg. Head
    )
    (:`SurfaceType3`
      (set `local.InDamageMultiplier` 0.7))
    (:`SurfaceType4`
      (set `local.InDamageMultiplier` 0.9)))
  (return (`KismetMathLibrary.SelectFloat` (* (`local.InDamageMultiplier`) 2.0) (`local.InDamageMultiplier`) (`local.InCriticalHit`))))

(fn `GetHitDecal`
  (params (PhysicMat :type "PhysicalMaterial Object Reference"))
  (returns (DecalMat :type "MaterialInterface Object Reference"))
  (switch `EPhysicalSurface` (`PhysicalMaterial.SurfaceType` PhysicMat)
    (:`SurfaceType_Default`
      (return "/Game/Defender/Demo/Materials/M_BulletDecal.M_BulletDecal"))
    (:`SurfaceType1`
      (return "/Game/Defender/Demo/Materials/M_BulletDecal.M_BulletDecal"))
    (:`SurfaceType2`
      (return "/Game/Defender/Demo/Materials/M_BulletDecal.M_BulletDecal"))
    (:`SurfaceType3`
      _)
    (:`SurfaceType4`
      _))
  (return "/Game/Defender/Demo/Materials/M_BulletDecal.M_BulletDecal"))

(fn `GetMeleeHitParticleEffect`
  (params (PhysicalMat :type "PhysicalMaterial Object Reference"))
  (returns (Particle :type "ParticleSystem Object Reference") (Scale :type "Vector Structure"))
  (switch `EPhysicalSurface` (`PhysicalMaterial.SurfaceType` PhysicalMat)
    (:`SurfaceType_Default`
      (return "/Game/Defender/Demo/Particles/P_Impact.P_Impact" (0.5 0.5 0.5)))
    (:`SurfaceType1`
      (return "/Game/Defender/Demo/Particles/P_body_bullet_impact.P_body_bullet_impact" (1.3 1.3 1.3)))
    (:`SurfaceType2`
      (return "/Game/Defender/Demo/Particles/P_body_bullet_impact.P_body_bullet_impact" (1.5 1.5 1.5)))
    (:`SurfaceType3`
      _)
    (:`SurfaceType4`
      _))
  (return "/Game/Defender/Demo/Particles/P_Sparks.P_Sparks" (1.5 1.5 1.5)))

(fn `GetMeleeHitSound`
  (params (PhysicalMat :type "PhysicalMaterial Object Reference"))
  (returns (Sound :type "SoundBase Object Reference"))
  (switch `EPhysicalSurface` (`PhysicalMaterial.SurfaceType` PhysicalMat)
    (:`SurfaceType_Default`
      (return "/Game/Defender/Demo/Audio/Impacts/SCue_Impt_Bullet_Default.SCue_Impt_Bullet_Default"))
    (:`SurfaceType1`
      (return "/Game/Defender/Demo/Audio/Impacts/SCue_SwordToFlesh.SCue_SwordToFlesh"))
    (:`SurfaceType2`
      (return "/Game/Defender/Demo/Audio/Impacts/SCue_SwordToFlesh.SCue_SwordToFlesh"))
    (:`SurfaceType3`
      _)
    (:`SurfaceType4`
      _))
  (return "/Game/Defender/Demo/Audio/Impacts/SCue_Impt_Metal_Melee.SCue_Impt_Metal_Melee"))

(fn `GetProjectileHitParticleEffect`
  (params (PhysicalMat :type "PhysicalMaterial Object Reference"))
  (returns (Particle :type "ParticleSystem Object Reference") (Scale :type "Vector Structure"))
  (switch `EPhysicalSurface` (`PhysicalMaterial.SurfaceType` PhysicalMat)
    (:`SurfaceType_Default`
      (return "/Game/Defender/Demo/Particles/P_Impact.P_Impact" (0.5 0.5 0.5)))
    (:`SurfaceType1`
      (return "/Game/Defender/Demo/Particles/P_body_bullet_impact.P_body_bullet_impact" (1.2 1.2 1.2)))
    (:`SurfaceType2`
      (return "/Game/Defender/Demo/Particles/P_body_bullet_impact.P_body_bullet_impact" (1.5 1.5 1.5)))
    (:`SurfaceType3`
      _)
    (:`SurfaceType4`
      _))
  (return "/Game/Defender/Demo/Particles/P_Sparks.P_Sparks" (1.0 1.0 1.0)))

(fn `GetProjectileHitSound`
  (params (Target :type "PhysicalMaterial Object Reference"))
  (returns (Sound :type "SoundBase Object Reference"))
  (switch `EPhysicalSurface` (`PhysicalMaterial.SurfaceType` Target)
    (:`SurfaceType_Default`
      (return "/Game/Defender/Demo/Audio/Impacts/SCue_Impt_Bullet_Default.SCue_Impt_Bullet_Default"))
    (:`SurfaceType1`
      (return "/Game/Defender/Demo/Audio/Impacts/SCue_Impt_Bullet_Flesh.SCue_Impt_Bullet_Flesh"))
    (:`SurfaceType2`
      (return "/Game/Defender/Demo/Audio/Impacts/SCue_Impt_Bullet_Flesh.SCue_Impt_Bullet_Flesh"))
    (:`SurfaceType3`
      _)
    (:`SurfaceType4`
      _))
  (return "/Game/Defender/Demo/Audio/Impacts/SCue_Impt_Bullet_Metal.SCue_Impt_Bullet_Metal"))