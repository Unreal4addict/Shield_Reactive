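; BP_FlickeringLight2 is a light Blueprint that flickers a point light's intensity during play.
; On BeginPlay, if flickering is enabled, it sets the timeline's play rate from FlickerRate and plays it.
; Each timeline update blends between low and high flicker intensities using the track value, then multiplies the result by brightness and a scale factor to set the light's intensity.
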(event `self.ReceiveBeginPlay`
  (if (`self.IsFlickerEnabled`)
    (`TimelineComponent.SetPlayRate` (`self.Timeline_0`) (`self.FlickerRate`))
    (bind (_direction _newtrack_0) (`Timeline|Timeline_0`)
      (:`Update`
        (`LightComponent.SetIntensity` (`self.PointLight`) (* (* (`self.LightBrightness`) (`self.LightScaleIntensity`)) (`KismetMathLibrary.Lerp` (`self.FlickerIntensityLow`) (`self.FlickerIntensityHigh`) _newtrack_0)))))))

(fn `UserConstructionScript`)