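; Base Blueprint for weapon loot in Defender, associating a WeaponClass with a SkeletalMesh component.
; BeginPlay and the construction script only call their parent implementations, and Tick is disabled.
; A deprecated, uncalled SetSkMesh function maps five weapon classes to meshes through nested branches, with the heavy machine gun reusing the assault rifle mesh.
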(event `self.ReceiveBeginPlay`
  (`parent.ReceiveBeginPlay`))

(fn `SetSkMesh`
  (if (== (`self.WeaponClass`) "/Game/Defender/Blueprints/Weapons/WeaponBP/BP_AssaultRifle.BP_AssaultRifle_C")
    (`SkinnedMeshComponent.SetSkinnedAssetAndUpdate` (`self.SkeletalMesh`) "/Game/Defender/Demo/Meshes/AssaultRifle/SK_AssaultRifle.SK_AssaultRifle" true)
    (elif (== (`self.WeaponClass`) "/Game/Defender/Blueprints/Weapons/WeaponBP/BP_PlasmaRifle.BP_PlasmaRifle_C")
      (`SkinnedMeshComponent.SetSkinnedAssetAndUpdate` (`self.SkeletalMesh`) "/Game/Defender/Demo/Meshes/PlasmaRifle/SK_PlasmaRifle.SK_PlasmaRifle" true)
      (elif (== (`self.WeaponClass`) "/Game/Defender/Blueprints/Weapons/WeaponBP/BP_HeavyMachineGun.BP_HeavyMachineGun_C")
        (`SkinnedMeshComponent.SetSkinnedAssetAndUpdate` (`self.SkeletalMesh`) "/Game/Defender/Demo/Meshes/AssaultRifle/SK_AssaultRifle.SK_AssaultRifle" true)
        (elif (== (`self.WeaponClass`) "/Game/Defender/Blueprints/Weapons/WeaponBP/BP_Launcher.BP_Launcher_C")
          (`SkinnedMeshComponent.SetSkinnedAssetAndUpdate` (`self.SkeletalMesh`) "/Game/Defender/Demo/Meshes/Launcher/SK_Launcher.SK_Launcher" true)
          (elif (== (`self.WeaponClass`) "/Game/Defender/Blueprints/Weapons/WeaponBP/BP_SniperRifle.BP_SniperRifle_C")
            (`SkinnedMeshComponent.SetSkinnedAssetAndUpdate` (`self.SkeletalMesh`) "/Game/Defender/Demo/Meshes/WraithGun/SK_WraithGun.SK_WraithGun" true)))))))

(fn `UserConstructionScript`
  (`parent.UserConstructionScript`))