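; BP_ActorSpawnerTarget is a spawn point that creates an actor of a chosen class at its own transform.
; SpawnSelectedClass always spawns, adjusting for collision if possible, stores and broadcasts the new actor, and prints an error if the class is invalid.
; It binds to the actor's HealthComp death event to rebroadcast deaths through its own dispatcher.
; DestroySpawnedActor removes the stored actor.
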(event `SpawnSelectedClass`
  (if (`KismetSystemLibrary.IsValidClass` (`self.ActorToSpawn`))
    (bind _returnvalue (`|SpawnActorFromClass` (`self.ActorToSpawn`) (`self.GetTransform`) "AdjustIfPossibleButAlwaysSpawn" "OverrideRootScale" null null))
    (bind _output_get (set `self.SpawnedActor` _returnvalue))
    (`/Engine/EditorBlueprintResources/StandardMacros.IsValid` _output_get
      (:`Is Valid`
        (`self.OnSpawnActor` (`self.SpawnedActor`))
        (bind _output_get_2 (set `self.SpawnedActorHealthComp` (`self.GetComponentByClass` (`self.SpawnedActor`) "/Game/Defender/Blueprints/Components/HealthComp.HealthComp_C")))
        (`/Engine/EditorBlueprintResources/StandardMacros.IsValid` _output_get_2
          (:`Is Valid`
            (add `/Game/Defender/Blueprints/Components/HealthComp.OnDeath` (`self.SpawnedActorHealthComp`) (delegate `OnDeath_Event_0`))))))
    (else
      (`KismetSystemLibrary.PrintString` "Error in one of your Spawner Target" true true (struct :`R` 0.320833 :`B` 0.025938 :`A` 1.0)))))

(event `OnDeath_Event_0`
  (params (BoneName :type Name) (ShotFromDirection :type "Vector Structure") (HitComponent :type "PrimitiveComponent Object Reference") (InstigatedBy :type "Controller Object Reference") (DamageCauser :type "Actor Object Reference"))
  (`self.OnSpawnedActorDeath` (`self.SpawnedActor`)))

(fn `DestroySpawnedActor`
  (`/Engine/EditorBlueprintResources/StandardMacros.IsValid` (`self.SpawnedActor`)
    (:`Is Valid`
      (`self.K2_DestroyActor` (`self.SpawnedActor`)))))

(fn `UserConstructionScript`)